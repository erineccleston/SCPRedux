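; Button_BP is an interactable button that opens the HeavyDoor_BP it is parented to.
; Overlapping its capsule enables player input and shows the character's interact icon, reversing both on exit.
; Pressing Interact copies the door's fail message and calls Open, then plays a press sound if the door is enabled.
; A disabled or missing parent door plays an alternate sound and queues the fail message on the player character.
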(event OnComponentBeginOverlap(Capsule)
  (params (OverlappedComponent :type Primitive%20Component%20Object%20Reference) (OtherActor :type Actor%20Object%20Reference) (OtherComp :type Primitive%20Component%20Object%20Reference) (OtherBodyIndex :type Integer) (bFromSweep :type Boolean) (SweepResult :type Hit%20Result%20Structure%20%28by%20ref%29))
  (bind _asscpredux_character_bp (Utilities|Casting|CastToSCPReduxCharacter_BP OtherActor))
  (Input|EnableInput (Game|GetPlayerController 0))
  (Widget|SetVisibility (Variables|/Game/SCP/Character/SCPReduxCharacter_BP.SCPReduxCharacter_BP_C|GetInteractIcon _asscpredux_character_bp) "Visible"))

(event OnComponentEndOverlap(Capsule)
  (params (OverlappedComponent :type Primitive%20Component%20Object%20Reference) (OtherActor :type Actor%20Object%20Reference) (OtherComp :type Primitive%20Component%20Object%20Reference) (OtherBodyIndex :type Integer))
  (bind _asscpredux_character_bp (Utilities|Casting|CastToSCPReduxCharacter_BP OtherActor))
  (Input|DisableInput (Game|GetPlayerController 0))
  (Widget|SetVisibility (Variables|/Game/SCP/Character/SCPReduxCharacter_BP.SCPReduxCharacter_BP_C|GetInteractIcon _asscpredux_character_bp) "Hidden"))

(event Input|ActionEvents|InputActionInteract
  (params (Key :type Key%20Structure :default "AnyKey"))
  (bind _returnvalue (Transformation|GetActorLocation))
  (:Pressed
    (bind _asheavy_door_bp (Utilities|Casting|CastToHeavyDoor_BP (Actor|GetParentActor))
      (:then
        (Variables|Default|SetFailMessage (Variables|/Game/SCP/Blueprints/HeavyDoor_BP.HeavyDoor_BP_C|GetFailMessage _asheavy_door_bp))
        (Default|Open _asheavy_door_bp)
        (if (Variables|/Game/SCP/Blueprints/HeavyDoor_BP.HeavyDoor_BP_C|GetDoorEnabled _asheavy_door_bp)
          (Audio|PlaySoundatLocation "/Game/SCP/Blueprints/Sounds/Button.Button" _returnvalue)
          (else
            (Audio|PlaySoundatLocation "/Game/SCP/Blueprints/Sounds/Button2.Button2" _returnvalue :!label _label)
            (bind _asscpredux_character_bp (Utilities|Casting|CastToSCPReduxCharacter_BP (Game|Player|GetPlayerPawn 0)))
            (Default|QueueMessage _asscpredux_character_bp (Variables|Default|GetFailMessage)))))
      (:CastFailed
        (goto _label)))))

(fn ConstructionScript)