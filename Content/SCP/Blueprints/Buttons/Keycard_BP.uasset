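; Keycard reader button that lets the player operate its linked parent only with sufficient security clearance.
; On Activate, it converts the player's active item to a card level and compares it with the first parent's clearance level.
; A pass runs the parent activation, while failures play a sound and queue a message for either low clearance or no keycard.
; After a pass or low-clearance attempt, the active item is cleared following a short delay.
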(event EventBeginPlay)

(event Collision|EventActorBeginOverlap
  (params (OtherActor :type Actor%20Object%20Reference)))

(event EventTick
  (params (DeltaSeconds :type Float%20%28single-precision%29)))

(event EventActivate
  (bind _returnvalue (Transformation|GetActorLocation))
  (bind _asscpredux_character_bp (Utilities|Casting|CastToSCPReduxCharacter_BP (Game|Player|GetPlayerPawn 0)))
  (bind _level (CallFunction|GetCardValue (Variables|/Game/SCP/Character/SCPReduxCharacter_BP.SCPReduxCharacter_BP_C|GetActiveItem _asscpredux_character_bp)))
  (if (>= _level (Variables|/Game/SCP/Blueprints/Doors/DoorBase_BP.DoorBase_BP_C|GetClearanceLevel (Utilities|Array|Get(acopy) (Variables|Default|GetParents))))
    (|CallParentFunction)
    (bind _asscpredux_character_bp_2 (Utilities|Casting|CastToSCPReduxCharacter_BP (Game|Player|GetPlayerPawn 0) :!label _label))
    (Utilities|FlowControl|Delay 0.1)
    (Variables|/Game/SCP/Character/SCPReduxCharacter_BP.SCPReduxCharacter_BP_C|SetActiveItem _asscpredux_character_bp_2 "NewEnumerator59")
    (elif (> _level -1)
      (Audio|PlaySoundatLocation (Variables|Default|GetFailSound) _returnvalue)
      (Default|QueueMessage _asscpredux_character_bp "A keycard with a higher security clearance is required to operate this door.")
      (goto _label)
      (else
        (Audio|PlaySoundatLocation "/Game/SCP/Blueprints/Sounds/Button.Button" _returnvalue)
        (Default|QueueMessage _asscpredux_character_bp "A keycard is required to operate this door.")))))

(fn ConstructionScript
  (|CallParentFunction))

(fn GetCardValue
  (params (Item :type Items_Enum%20Enum))
  (Utilities|FlowControl|Sequence
    (:then_0
      (switch Utilities|FlowControl|Switch|SwitchonItems_Enum Item
        (:NewEnumerator3
          (return 1))
        (:NewEnumerator4
          (return 2))
        (:NewEnumerator5
          (return 3))
        (:NewEnumerator6
          (return 4))
        (:NewEnumerator7
          (return 5))
        (:NewEnumerator8
          (return 6))
        (:NewEnumerator69
          (return 0))))
    (:then_1
      (return -1))))