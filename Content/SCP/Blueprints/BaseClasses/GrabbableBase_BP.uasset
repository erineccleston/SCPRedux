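; Base actor for grabbable objects the SCP player can interact with and hold.
; While the player overlaps its capsule, Tick uses screen projection and a recently-rendered check to add or remove it from InteractablesInRange, gated by DoOnce nodes.
; Activate and Deactivate toggle the grab, and Tick derives a scaled camera rotation delta.
; Empty WhileGrabbed and SettlingBehavior events serve as hooks for held and release behavior.
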(event OnComponentBeginOverlap(Capsule)
  (params (OverlappedComponent :type Primitive%20Component%20Object%20Reference) (OtherActor :type Actor%20Object%20Reference) (OtherComp :type Primitive%20Component%20Object%20Reference) (OtherBodyIndex :type Integer) (bFromSweep :type Boolean) (SweepResult :type Hit%20Result%20Structure%20%28by%20ref%29))
  (Utilities|Casting|CastToSCPReduxCharacter_BP OtherActor)
  (Variables|Default|SetInRange true))

(event OnComponentEndOverlap(Capsule)
  (params (OverlappedComponent :type Primitive%20Component%20Object%20Reference) (OtherActor :type Actor%20Object%20Reference) (OtherComp :type Primitive%20Component%20Object%20Reference) (OtherBodyIndex :type Integer))
  (Utilities|Casting|CastToSCPReduxCharacter_BP OtherActor)
  (Variables|Default|SetInRange false)
  (Variables|Default|SetGrabbed false)
  (CallFunction|RemovefromInteractables))

(event Custom|ResetAdd
  (Utilities|FlowControl|DoOnce false) ; enters at Reset
)

(event Custom|WhileGrabbed)

(event Custom|SettlingBehavior)

(event EventActivate
  (Variables|Default|SetGrabbed true)
  (Variables|Default|SetPreviousSelfRotation (Transformation|GetWorldRotation (Variables|Default|GetBody)))
  (Variables|Default|SetPreviousPlayerRotation (Transformation|GetWorldRotation (Variables|/Script/SCPRedux.SCPReduxCharacter|GetFirstPersonCameraComponent (.AsSCPRedux%20Character%20BP (Utilities|Casting|CastToSCPReduxCharacter_BP (Game|Player|GetPlayerPawn 0)))))))

(event EventDeactivate
  (Variables|Default|SetGrabbed false)
  (CallFunction|SettlingBehavior))

(event EventTick
  (params (DeltaSeconds :type Float%20%28single-precision%29))
  (if (and (Variables|Default|GetInRange) (Variables|Default|GetEnabled))
    (Utilities|FlowControl|Sequence
      (:then_0
        (bind _centered (CallFunction|IsCentered))
        (if (and (not _centered) (not (Variables|Default|GetGrabbed)))
          _
          (elif (not (Class|Actor|WasRecentlyRendered 0.2))
            _
            (else
              (Utilities|FlowControl|DoOnce false
                (:Completed
                  (Utilities|Array|Add (Variables|/Game/SCP/Character/SCPReduxCharacter_BP.SCPReduxCharacter_BP_C|GetInteractablesInRange (.AsSCPRedux%20Character%20BP (Utilities|Casting|CastToSCPReduxCharacter_BP (Game|Player|GetPlayerPawn 0)))) self)
                  (goto _label Reset))))))
        (Utilities|FlowControl|DoOnce false :!label _label
          (:Completed
            (CallFunction|RemovefromInteractables)
            (Variables|Default|SetGrabbed false))))
      (:then_1
        (Variables|Default|SetPlayerRotDelta (* (* (Math|Rotator|Delta(Rotator) (Transformation|GetWorldRotation (Variables|/Script/SCPRedux.SCPReduxCharacter|GetFirstPersonCameraComponent (.AsSCPRedux%20Character%20BP (Utilities|Casting|CastToSCPReduxCharacter_BP (Game|Player|GetPlayerPawn 0))))) (Variables|Default|GetPreviousPlayerRotation)) DeltaSeconds) (Variables|Default|GetTurnSpeed)))
        (Variables|Default|SetPreviousPlayerRotation (Transformation|GetWorldRotation (Variables|/Script/SCPRedux.SCPReduxCharacter|GetFirstPersonCameraComponent (.AsSCPRedux%20Character%20BP (Utilities|Casting|CastToSCPReduxCharacter_BP (Game|Player|GetPlayerPawn 0))))))
        (if (Variables|Default|GetGrabbed)
          (CallFunction|WhileGrabbed))))))

(fn ConstructionScript
  (|CallParentFunction))

(fn RemovefromInteractables
  (bind _asscpredux_character_bp (Utilities|Casting|CastToSCPReduxCharacter_BP (Game|Player|GetPlayerPawn 0)))
  (Utilities|Array|RemoveItem (Variables|/Game/SCP/Character/SCPReduxCharacter_BP.SCPReduxCharacter_BP_C|GetInteractablesInRange _asscpredux_character_bp) self)
  (CallFunction|ResetAdd))

(fn IsCentered
  (bind _returnvalue (Game|GetPlayerController 0))
  (bind _returnvalue_2 (Viewport|GetViewportSize))
  (bind _returnvalue_3 (Transformation|GetActorLocation))
  (bind _visualsize (Variables|Default|GetVisualSize))
  (bind _screenposition (Class|GameplayStatics|ProjectWorldtoScreen _returnvalue _returnvalue_3 false))
  (return (and (Math|Float|NearlyEqual(Float) (.x _screenposition) (/ (.x _returnvalue_2) 2.0) _visualsize) (Math|Float|NearlyEqual(Float) (.y _screenposition) (/ (.y _returnvalue_2) 2.0) _visualsize))))