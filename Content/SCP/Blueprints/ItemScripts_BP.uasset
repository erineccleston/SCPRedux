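; Item script library for an SCP game that applies each item type's effect to the player character when used.
; ScriptSwitch makes keys, keycards and hands the active item, toggles the stamina-capping 714 ring, or turns the 523 fake card into Keycard 0.
; WearableSwitch resets, then toggles worn gear, setting overlays, stamina regen and NVG fog distance.
; ScriptSwitchBackup6/4 holds older dispatch logic; the hazmat stamina change is disconnected.
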(fn ScriptSwitch
  (params (Type :type Items_Enum%20Enum))
  (switch Utilities|FlowControl|Switch|SwitchonItems_Enum Type
    (:NewEnumerator0
      (Callable|WearableSwitch Type :!label _label))
    (:NewEnumerator1
      (goto _label))
    (:NewEnumerator2
      (goto _label))
    (:NewEnumerator3
      (Helper|SetActiveItem Type :!label _label_2))
    (:NewEnumerator4
      (goto _label_2))
    (:NewEnumerator5
      (goto _label_2))
    (:NewEnumerator6
      (goto _label_2))
    (:NewEnumerator7
      (goto _label_2))
    (:NewEnumerator8
      (goto _label_2))
    (:NewEnumerator21
      (Callable|WearableSwitch Type :!label _label_3))
    (:NewEnumerator22
      (goto _label_3))
    (:NewEnumerator23
      (goto _label_3))
    (:NewEnumerator30
      (Helper|SetActiveItem Type :!label _label_4))
    (:NewEnumerator31
      (goto _label_4))
    (:NewEnumerator33
      (Callable|WearableSwitch Type :!label _label_5))
    (:NewEnumerator34
      (goto _label_5))
    (:NewEnumerator35
      (goto _label_5))
    (:NewEnumerator38
      (goto _label_5))
    (:NewEnumerator41
      (Scripts|Toggle714Ring))
    (:NewEnumerator42
      (Helper|SetActiveItem Type :!label _label_6))
    (:NewEnumerator46
      (goto _label_6))
    (:NewEnumerator69
      (Helper|SetActiveItem Type))
    (:NewEnumerator70
      (Scripts|523Script))))

(fn GetAttributes
  (params (Type :type Items_Enum%20Enum))
  (bind _enumattribmap (LocalVariables|GetEnumAttribMap))
  (bind (_value _returnvalue) (Utilities|Map|Find _enumattribmap Type))
  (return _value _returnvalue))

(fn ApplySuperGasMaskEffect
  (Variables|/Game/SCP/Character/SCPReduxCharacter_BP.SCPReduxCharacter_BP_C|SetStaminaRegenMultiplier (Helper|GetPlayerChar) 1.25e+03))

(fn GetPlayerChar
  (return (.AsSCPRedux%20Character%20BP (Utilities|Casting|CastToSCPReduxCharacter_BP (Game|Player|GetPlayerPawn 0)))))

(fn ApplyHeadgearOverlay
  (params (Texture :type Material%20Object%20Reference) (Color :type Linear%20Color%20Structure))
  (bind _playerchar (Helper|GetPlayerChar))
  (bind _wearableoverlay (Variables|/Game/SCP/Character/SCPReduxCharacter_BP.SCPReduxCharacter_BP_C|GetWearableOverlay _playerchar))
  (Variables|/Game/SCP/HUD/WearableOverlay.WearableOverlay_C|SetTexture _wearableoverlay Texture)
  (Variables|/Game/SCP/HUD/WearableOverlay.WearableOverlay_C|SetColor _wearableoverlay Color))

(fn Toggle714Ring
  (bind _playerchar (Helper|GetPlayerChar))
  (if (Variables|/Game/SCP/Character/SCPReduxCharacter_BP.SCPReduxCharacter_BP_C|Get714RingEquipped _playerchar)
    (Variables|/Game/SCP/Character/SCPReduxCharacter_BP.SCPReduxCharacter_BP_C|SetMaxStamina _playerchar 1e+02)
    (else
      (Variables|/Game/SCP/Character/SCPReduxCharacter_BP.SCPReduxCharacter_BP_C|SetMaxStamina _playerchar 1e+01)
      (Variables|/Game/SCP/Character/SCPReduxCharacter_BP.SCPReduxCharacter_BP_C|SetStaminaValue _playerchar 1e+01)))
  (Variables|/Game/SCP/Character/SCPReduxCharacter_BP.SCPReduxCharacter_BP_C|Set714RingEquipped _playerchar (not (Variables|/Game/SCP/Character/SCPReduxCharacter_BP.SCPReduxCharacter_BP_C|Get714RingEquipped _playerchar))))

(fn SetActiveItem
  (params (Type :type Items_Enum%20Enum))
  (Variables|/Game/SCP/Character/SCPReduxCharacter_BP.SCPReduxCharacter_BP_C|SetActiveItem (Helper|GetPlayerChar) Type))

(fn ResetAllWearables
  (bind _playerchar (Helper|GetPlayerChar))
  (Variables|/Game/SCP/HUD/WearableOverlay.WearableOverlay_C|SetColor (Variables|/Game/SCP/Character/SCPReduxCharacter_BP.SCPReduxCharacter_BP_C|GetWearableOverlay _playerchar) "(R=0.000000,G=0.000000,B=0.000000,A=0.000000)")
  (Variables|/Game/SCP/Character/SCPReduxCharacter_BP.SCPReduxCharacter_BP_C|SetWornItem _playerchar "NewEnumerator59")
  (Variables|/Game/SCP/Character/SCPReduxCharacter_BP.SCPReduxCharacter_BP_C|SetStaminaRegenMultiplier _playerchar 0.0)
  (Helper|SetFogStartDistance 1.75e+03))

(fn SetWornItem
  (params (Type :type Items_Enum%20Enum))
  (Variables|/Game/SCP/Character/SCPReduxCharacter_BP.SCPReduxCharacter_BP_C|SetWornItem (Helper|GetPlayerChar) Type))

(fn GenericGasMask
  (Helper|ApplyHeadgearOverlay "/Game/SCP/HUD/Textures/GasmaskOverlay_Mat.GasmaskOverlay_Mat" "(R=1.000000,G=1.000000,B=1.000000,A=1.000000)"))

(fn ApplyHazmatStamina)

(fn WearableSwitch
  (params (Type :type Items_Enum%20Enum))
  (LocalVariables|SetNewItem Type)
  (LocalVariables|SetOldItem (Variables|/Game/SCP/Character/SCPReduxCharacter_BP.SCPReduxCharacter_BP_C|GetWornItem (Helper|GetPlayerChar)))
  (Helper|ResetAllWearables)
  (if (Utilities|Enum|NotEqual(Enum) (LocalVariables|GetNewItem) (LocalVariables|GetOldItem))
    (Helper|SetWornItem (LocalVariables|GetNewItem))
    (switch Utilities|FlowControl|Switch|SwitchonItems_Enum (LocalVariables|GetNewItem)
      (:NewEnumerator0
        (Scripts|GenericGasMask))
      (:NewEnumerator1
        (Scripts|GenericGasMask)
        (Scripts|ApplySuperGasMaskEffect))
      (:NewEnumerator2
        (Scripts|GenericGasMask))
      (:NewEnumerator21
        (Scripts|GenericHazmat))
      (:NewEnumerator22
        (Scripts|GenericHazmat))
      (:NewEnumerator23
        (Scripts|GenericHazmat)
        (Scripts|ApplySuperGasMaskEffect))
      (:NewEnumerator33
        (Scripts|GenericNVG "(R=0.000000,G=1.000000,B=0.000000,A=1.000000)"))
      (:NewEnumerator34
        (Scripts|GenericNVG "(R=0.000000,G=0.000000,B=1.000000,A=1.000000)"))
      (:NewEnumerator35
        (Scripts|GenericNVG "(R=1.000000,G=0.000000,B=0.000000,A=1.000000)"))
      (:NewEnumerator38
        (Helper|ApplyHeadgearOverlay "/Game/SCP/HUD/Textures/SpecsOverlay_Mat.SpecsOverlay_Mat" "(R=1.000000,G=1.000000,B=1.000000,A=1.000000)")))))

(fn ScriptSwitchBackup6/4
  (params (Type :type Items_Enum%20Enum))
  (switch Utilities|FlowControl|Switch|SwitchonItems_Enum Type
    (:NewEnumerator0
      (Helper|ResetAllWearables)
      (Scripts|GenericGasMask)
      (Helper|SetWornItem "NewEnumerator0"))
    (:NewEnumerator1
      (Helper|ResetAllWearables)
      (Scripts|ApplySuperGasMaskEffect)
      (Scripts|GenericGasMask)
      (Helper|SetWornItem "NewEnumerator1"))
    (:NewEnumerator2
      (Helper|ResetAllWearables)
      (Scripts|GenericGasMask)
      (Helper|SetWornItem "NewEnumerator2"))
    (:NewEnumerator3
      (Helper|SetActiveItem "NewEnumerator3"))
    (:NewEnumerator4
      (Helper|SetActiveItem "NewEnumerator4"))
    (:NewEnumerator5
      (Helper|SetActiveItem "NewEnumerator5"))
    (:NewEnumerator6
      (Helper|SetActiveItem "NewEnumerator6"))
    (:NewEnumerator7
      (Helper|SetActiveItem "NewEnumerator7"))
    (:NewEnumerator8
      (Helper|SetActiveItem "NewEnumerator8"))
    (:NewEnumerator21
      (Helper|ResetAllWearables)
      (Scripts|ApplyHazmatStamina)
      (Scripts|GenericGasMask)
      (Helper|SetWornItem "NewEnumerator21"))
    (:NewEnumerator22
      (Helper|ResetAllWearables)
      (Scripts|ApplySuperGasMaskEffect)
      (Scripts|GenericGasMask)
      (Helper|SetWornItem "NewEnumerator22"))
    (:NewEnumerator23
      (Helper|ResetAllWearables)
      (Scripts|ApplyHazmatStamina)
      (Scripts|GenericGasMask)
      (Helper|SetWornItem "NewEnumerator23"))
    (:NewEnumerator30
      (Helper|SetActiveItem "NewEnumerator30"))
    (:NewEnumerator31
      (Helper|SetActiveItem "NewEnumerator31"))
    (:NewEnumerator33
      (Helper|ResetAllWearables)
      (Helper|ApplyHeadgearOverlay "/Game/SCP/HUD/Textures/NightVisionOverlay_Mat.NightVisionOverlay_Mat" "(R=0.000000,G=1.000000,B=0.000000,A=1.000000)"))
    (:NewEnumerator34
      (Helper|ResetAllWearables)
      (Helper|ApplyHeadgearOverlay "/Game/SCP/HUD/Textures/NightVisionOverlay_Mat.NightVisionOverlay_Mat" "(R=1.000000,G=0.000000,B=0.000000,A=1.000000)"))
    (:NewEnumerator35
      (Helper|ResetAllWearables)
      (Helper|ApplyHeadgearOverlay "/Game/SCP/HUD/Textures/NightVisionOverlay_Mat.NightVisionOverlay_Mat" "(R=0.000000,G=0.000000,B=1.000000,A=1.000000)"))
    (:NewEnumerator41
      (Scripts|Toggle714Ring))
    (:NewEnumerator42
      (Helper|SetActiveItem "NewEnumerator42"))))

(fn GenericHazmat
  (Scripts|ApplyHazmatStamina)
  (Scripts|GenericGasMask))

(fn GenericNVG
  (params (Color :type Linear%20Color%20Structure))
  (Helper|ApplyHeadgearOverlay "/Game/SCP/HUD/Textures/NightVisionOverlay_Mat.NightVisionOverlay_Mat" Color)
  (Helper|SetFogStartDistance 3.5e+03))

(fn SetFogStartDistance
  (params (Distance :type Float%20%28single-precision%29))
  (bind _outactors (Actor|GetAllActorsOfClass 0 "/Script/Engine.ExponentialHeightFog"))
  (if (> (Utilities|Array|Length _outactors) 0)
    (Class|ExponentialHeightFogComponent|SetStartDistance (Variables|/Script/Engine.ExponentialHeightFog|GetComponent (Utilities|Array|Get(acopy) _outactors)) Distance)
    (else
      (Development|PrintString 0 "No ExponentialHeightFog Actor found."))))

(fn 523Script
  (bind _playerchar (Helper|GetPlayerChar))
  (bind _inventory (Variables|/Game/SCP/Character/SCPReduxCharacter_BP.SCPReduxCharacter_BP_C|GetInventory _playerchar))
  (Utilities|Array|SetArrayElem _inventory (Utilities|Array|FindItem _inventory "NewEnumerator70") "NewEnumerator69")
  (Helper|SetActiveItem "NewEnumerator69"))