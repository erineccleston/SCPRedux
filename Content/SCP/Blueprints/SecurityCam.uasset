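; SecurityCam is a security camera actor that rotates between two limits 45 degrees either side of its starting rotation.
; BeginPlay computes both limits, and Tick plays the Rotation timeline, whose alpha lerps the actor between them along the shortest path.
; The construction script uses RecordsWorld to toggle the scene capture component's visibility and, when enabled, assigns its render target and maximum view distance.
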(event EventBeginPlay
  (bind _returnvalue (Transformation|GetActorRotation))
  (Variables|Default|SetLeftRotation (Math|Rotator|CombineRotators _returnvalue "0,45.000000, 0"))
  (Variables|Default|SetRightRotation (Math|Rotator|CombineRotators _returnvalue "0,-45.000000, 0")))

(event EventTick
  (params (DeltaSeconds :type Float%20%28single-precision%29))
  (bind _alpha (Timeline|Rotation Play)
    (:Update
      (Transformation|SetActorRotation (Math|Rotator|Lerp(Rotator) (Variables|Default|GetLeftRotation) (Variables|Default|GetRightRotation) _alpha true)))))

(fn ConstructionScript
  (bind _recordsworld (Variables|Default|GetRecordsWorld))
  (Rendering|SetVisibility (Variables|Default|GetSceneCaptureComponent) _recordsworld false)
  (if _recordsworld
    (Variables|/Script/Engine.SceneCaptureComponent2D|SetTextureTarget (Variables|Default|GetSceneCaptureComponent) (Variables|Default|GetSceneCaptureTexture))
    (Variables|/Script/Engine.SceneCaptureComponent|SetMaxViewDistanceOverride (Variables|Default|GetSceneCaptureComponent) (Variables|Default|GetMaxViewDistance))))