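; HUD Blueprint that draws on-screen text messages for the SCP game.
; QueueDrawText appends to TextQueue, and DrawHUD draws the front entry in the lower center each frame, using a Delay to remove it after about three seconds.
; A separate DisplayMessage event uses a Gate around larger centered text, but nothing feeds the gate's Enter.
; BlinkStaminaMeters widget creation is present but unconnected, so it never runs.
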(event Custom|Queue%20Draw%20Text
  (params (Message :type String))
  (Utilities|Array|Add (Variables|Default|GetTextQueue) Message))

(event Custom|Display%20Message
  (params (Draw :type Boolean) (Text :type String))
  (bind _returnvalue (Viewport|GetViewportSize))
  (if Draw
    (Utilities|FlowControl|Gate true :!label _label ; enters at Open
      (:Exit
        (HUD|DrawText Text "(R=1.000000,G=1.000000,B=1.000000,A=1.000000)" (/ (.x _returnvalue) 2.0) (/ (.y _returnvalue) 2.0) "/Game/SCP/Menu/Fonts/cour_Font.cour_Font" 2.0 false)
        (Utilities|FlowControl|Delay 2.0)
        (goto _label Close)))
    (else
      (goto _label Close))))

(event EventBeginPlay)

(event Collision|EventActorBeginOverlap
  (params (OtherActor :type Actor%20Object%20Reference)))

(event EventTick
  (params (DeltaSeconds :type Float%20%28single-precision%29)))

(event EventDrawHUD
  (params (SizeX :type Integer) (SizeY :type Integer))
  (bind _returnvalue (Viewport|GetViewportSize))
  (bind _textqueue (Variables|Default|GetTextQueue))
  (if (> (Utilities|Array|Length _textqueue) 0)
    (HUD|DrawText (Utilities|Array|Get(acopy) _textqueue) "(R=1.000000,G=1.000000,B=1.000000,A=1.000000)" (* (.x _returnvalue) 0.5) (* (.y _returnvalue) 0.7) "/Game/SCP/Menu/Fonts/cour_Font.cour_Font" 0.3 false)
    (Utilities|FlowControl|Delay 3.0)
    (Utilities|Array|RemoveIndex _textqueue)))

(fn ConstructionScript)