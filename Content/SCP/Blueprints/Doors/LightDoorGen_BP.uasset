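; Light door actor for the SCP game, operated by two child-actor buttons, with an optional jumpscare mode.
; The construction script registers the door as each button's parent and sets StartOpen when JumpscareDoor is enabled.
; In that mode, the player's first overlap with JumpscareCollider calls Open and plays a horror door sound at the door, guarded by a DoOnce.
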(event OnComponentBeginOverlap(JumpscareCollider)
  (params (OverlappedComponent :type Primitive%20Component%20Object%20Reference) (OtherActor :type Actor%20Object%20Reference) (OtherComp :type Primitive%20Component%20Object%20Reference) (OtherBodyIndex :type Integer) (bFromSweep :type Boolean) (SweepResult :type Hit%20Result%20Structure%20%28by%20ref%29))
  (if (Variables|Default|GetJumpscareDoor)
    (Utilities|Casting|CastToSCPReduxCharacter_BP OtherActor)
    (Utilities|FlowControl|DoOnce false
      (:Completed
        (CallFunction|Open)
        (Audio|PlaySoundatLocation "/Game/SCP/Blueprints/Sounds/HorrorDoor.HorrorDoor" (Transformation|GetActorLocation))))))

(event EventBeginPlay
  (|CallParentFunction))

(event Collision|EventActorBeginOverlap
  (params (OtherActor :type Actor%20Object%20Reference)))

(event EventTick
  (params (DeltaSeconds :type Float%20%28single-precision%29)))

(fn ConstructionScript
  (|CallParentFunction)
  (bind _asbutton_base_bp (Utilities|Casting|CastToButtonBase_BP (Variables|/Script/Engine.ChildActorComponent|GetChildActor (Variables|Default|GetButton1))))
  (Variables|/Game/SCP/Blueprints/BaseClasses/ButtonBase_BP.ButtonBase_BP_C|SetParentDoor _asbutton_base_bp self)
  (bind _asbutton_base_bp_2 (Utilities|Casting|CastToButtonBase_BP (Variables|/Script/Engine.ChildActorComponent|GetChildActor (Variables|Default|GetButton2))))
  (Variables|/Game/SCP/Blueprints/BaseClasses/ButtonBase_BP.ButtonBase_BP_C|SetParentDoor _asbutton_base_bp_2 self)
  (if (Variables|Default|GetJumpscareDoor)
    (Variables|Default|SetStartOpen true)))