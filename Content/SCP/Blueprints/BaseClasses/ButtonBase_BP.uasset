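; Base keypad button that opens doors when activated and registers itself with the player character as interactable while inside its capsule.
; It opens its parent actor door or, lacking one, every door in its Parents array, gated only by the first door's enabled state.
; Success or failure selects the interact sound and queued player message.
; A dynamic material lets ChangeDisplay swap the keypad's in/out textures.
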(event OnComponentBeginOverlap(Capsule)
  (params (OverlappedComponent :type Primitive%20Component%20Object%20Reference) (OtherActor :type Actor%20Object%20Reference) (OtherComp :type Primitive%20Component%20Object%20Reference) (OtherBodyIndex :type Integer) (bFromSweep :type Boolean) (SweepResult :type Hit%20Result%20Structure%20%28by%20ref%29))
  (bind _asscpredux_character_bp (Utilities|Casting|CastToSCPReduxCharacter_BP OtherActor))
  (Utilities|Array|Add (Variables|/Game/SCP/Character/SCPReduxCharacter_BP.SCPReduxCharacter_BP_C|GetInteractablesInRange _asscpredux_character_bp) self))

(event OnComponentEndOverlap(Capsule)
  (params (OverlappedComponent :type Primitive%20Component%20Object%20Reference) (OtherActor :type Actor%20Object%20Reference) (OtherComp :type Primitive%20Component%20Object%20Reference) (OtherBodyIndex :type Integer))
  (bind _asscpredux_character_bp (Utilities|Casting|CastToSCPReduxCharacter_BP OtherActor))
  (Utilities|Array|RemoveItem (Variables|/Game/SCP/Character/SCPReduxCharacter_BP.SCPReduxCharacter_BP_C|GetInteractablesInRange _asscpredux_character_bp) self))

(event EventActivate
  (bind _returnvalue (Game|Player|GetPlayerPawn 0))
  (bind _parents (Variables|Default|GetParents))
  (Utilities|IsValid (Variables|Default|GetParentDoor)
    (:Is%20Valid
      (if (Variables|/Game/SCP/Blueprints/BaseClasses/DoorBase_BP.DoorBase_BP_C|GetDoorEnabled (Variables|Default|GetParentDoor))
        (Default|Open (Variables|Default|GetParentDoor))
        (Variables|Default|SetInteractSound (Variables|Default|GetSuccessSound) :!label _label)
        (bind _asscpredux_character_bp (Utilities|Casting|CastToSCPReduxCharacter_BP _returnvalue))
        (Default|QueueMessage _asscpredux_character_bp (Variables|Default|GetSuccessMessage))
        (else
          (Variables|Default|SetInteractSound (Variables|Default|GetFailSound) :!label _label_2)
          (bind _asscpredux_character_bp_2 (Utilities|Casting|CastToSCPReduxCharacter_BP _returnvalue))
          (Default|QueueMessage _asscpredux_character_bp_2 (Variables|Default|GetFailMessage)))))
    (:Is%20Not%20Valid
      (if (> (Utilities|Array|Length _parents) 0)
        (if (Variables|/Game/SCP/Blueprints/BaseClasses/DoorBase_BP.DoorBase_BP_C|GetDoorEnabled (Utilities|Array|Get(acopy) _parents))
          (for _array_element _parents
            (Default|Open _array_element))
          (goto _label)
          (else
            (goto _label_2)))
        (else
          (goto _label_2)))))
  (|CallParentFunction))

(event EventBeginPlay
  (bind _asdoor_base_bp (Utilities|Casting|CastToDoorBase_BP (Actor|GetParentActor)))
  (Variables|Default|SetParentDoor _asdoor_base_bp)
  (CallFunction|ChangeDisplay false))

(fn ConstructionScript
  (bind _returnvalue (Rendering|Material|CreateDynamicMaterialInstance "/Game/SCP/Blueprints/Materials/KeyPadEmis.KeyPadEmis" :!class /Script/Engine.KismetMaterialLibrary))
  (bind _output_get (Variables|Default|SetDynMatInst _returnvalue))
  (Rendering|Material|SetMaterial (Variables|Default|GetBody) 0 _output_get))

(fn ChangeDisplay
  (params (IsOpen :type Boolean))
  (bind _dynmatinst (Variables|Default|GetDynMatInst))
  (if IsOpen
    (Rendering|Material|SetTextureParameterValue _dynmatinst "SCPTex" "/Game/SCP/Blueprints/Materials/Textures/KeyPadOut.KeyPadOut")
    (else
      (Rendering|Material|SetTextureParameterValue _dynmatinst "SCPTex" "/Game/SCP/Blueprints/Materials/Textures/KeyPadIn.KeyPadIn"))))