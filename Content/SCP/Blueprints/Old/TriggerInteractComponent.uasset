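; Actor component that makes its owner, expected to be a ButtonBase_BP, interactable when the SCPRedux player character enters its capsule trigger.
; Begin and end overlap adjust the character's ItemsInRange count, toggle the owner's input, and start or stop icon tracking.
; While tracking, Tick projects the button body onto the screen and moves the player's hand icon there, clamped within screen margins, or centred when projection fails.
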(event Custom|OnComponentBeginOverlap_Event_0
  (params (OverlappedComponent :type Primitive%20Component%20Object%20Reference) (OtherActor :type Actor%20Object%20Reference) (OtherComp :type Primitive%20Component%20Object%20Reference) (OtherBodyIndex :type Integer) (bFromSweep :type Boolean) (SweepResult :type Hit%20Result%20Structure%20%28by%20ref%29))
  (bind _asscpredux_character_bp (Utilities|Casting|CastToSCPReduxCharacter_BP OtherActor))
  (Math|Integer|IncrementInt (Variables|/Game/SCP/Character/SCPReduxCharacter_BP.SCPReduxCharacter_BP_C|GetItemsInRange _asscpredux_character_bp)
    (:%20%20
      (Input|EnableInput (Components|GetOwner) (Game|GetPlayerController 0))
      (Variables|/Game/SCP/HUD/InteractIcon.InteractIcon_C|SetImage (Variables|Default|GetIconRef) "/Game/SCP/HUD/Textures/handsymbol.handsymbol")
      (Variables|Default|SetMoveInteractIcon true))))

(event Custom|OnComponentEndOverlap_Event_0
  (params (OverlappedComponent :type Primitive%20Component%20Object%20Reference) (OtherActor :type Actor%20Object%20Reference) (OtherComp :type Primitive%20Component%20Object%20Reference) (OtherBodyIndex :type Integer))
  (bind _asscpredux_character_bp (Utilities|Casting|CastToSCPReduxCharacter_BP OtherActor))
  (Math|Integer|DecrementInt (Variables|/Game/SCP/Character/SCPReduxCharacter_BP.SCPReduxCharacter_BP_C|GetItemsInRange _asscpredux_character_bp)
    (:%20%20
      (Input|DisableInput (Components|GetOwner) (Game|GetPlayerController 0))
      (Variables|Default|SetMoveInteractIcon false))))

(event EventBeginPlay
  (bind _returnvalue (Components|GetOwner))
  (bind _returnvalue_2 (Actor|GetComponentbyClass _returnvalue "/Script/Engine.CapsuleComponent"))
  (Collision|AssignOnComponentBeginOverlap _returnvalue_2 (delegate Custom|OnComponentBeginOverlap_Event_0))
  (Collision|AssignOnComponentEndOverlap _returnvalue_2 (delegate Custom|OnComponentEndOverlap_Event_0))
  (bind _asscpredux_character_bp (Utilities|Casting|CastToSCPReduxCharacter_BP (Game|Player|GetPlayerPawn 0)))
  (Variables|Default|SetIconRef (Variables|/Game/SCP/Character/SCPReduxCharacter_BP.SCPReduxCharacter_BP_C|GetInteractIcon _asscpredux_character_bp)))

(event EventTick
  (params (DeltaSeconds :type Float%20%28single-precision%29))
  (bind _returnvalue (Viewport|GetViewportSize))
  (bind _returnvalue_2 (Class|WidgetLayoutLibrary|GetViewportScale))
  (bind _returnvalue_3 (Viewport|GetViewportSize))
  (bind _returnvalue_4 (Class|WidgetLayoutLibrary|GetViewportScale))
  (bind _iconref (Variables|Default|GetIconRef))
  (bind _returnvalue_5 (/ (.x _returnvalue_3) _returnvalue_4))
  (bind _returnvalue_6 (/ (.y _returnvalue_3) _returnvalue_4))
  (if (Variables|Default|GetMoveInteractIcon)
    (bind _asbutton_base_bp (Utilities|Casting|CastToButtonBase_BP (Components|GetOwner)))
    (if (.ReturnValue (Class|WidgetLayoutLibrary|ProjectWorldLocationtoWidgetPosition (Game|GetPlayerController 0) (Transformation|GetWorldLocation (Variables|/Game/SCP/Blueprints/BaseClasses/InteractableBase_BP.InteractableBase_BP_C|GetBody _asbutton_base_bp))))
      (Class|Widget|SetRenderTranslation _iconref (Math|Vector2D|MakeVector2D (- (Math|Float|Clamp(Float) (.x (.ScreenPosition (Class|WidgetLayoutLibrary|ProjectWorldLocationtoWidgetPosition (Game|GetPlayerController 0) (Transformation|GetWorldLocation (Variables|/Game/SCP/Blueprints/BaseClasses/InteractableBase_BP.InteractableBase_BP_C|GetBody _asbutton_base_bp))))) (* _returnvalue_5 0.1) (* _returnvalue_5 0.9)) 32.0) (- (Math|Float|Clamp(Float) (.y (.ScreenPosition (Class|WidgetLayoutLibrary|ProjectWorldLocationtoWidgetPosition (Game|GetPlayerController 0) (Transformation|GetWorldLocation (Variables|/Game/SCP/Blueprints/BaseClasses/InteractableBase_BP.InteractableBase_BP_C|GetBody _asbutton_base_bp))))) (* _returnvalue_6 0.15) (* _returnvalue_6 0.85)) 32.0)))
      (else
        (Class|Widget|SetRenderTranslation _iconref (Math|Vector2D|MakeVector2D (- (/ (/ (.x _returnvalue) _returnvalue_2) 2.0) 32.0) (- (/ (/ (.y _returnvalue) _returnvalue_2) 2.0) 32.0)))))))