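; Grabbable two-position lever that plays a flip sound and notifies its parent RoomBase_BP of its up/down state.
; While grabbed, player pitch input rolls the body, reverting at the tilt limit; SettlingBehavior eases it to the nearer end with a timeline.
; Two cross-resetting DoOnce gates make each flip fire once.
; StartDown sets the initial pose and feeds the gates' starting state.
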(event EventWhileGrabbed
  (bind _startdown (Variables|Default|GetStartDown))
  (Variables|Default|SetOldRot (Transformation|GetWorldRotation (Variables|Default|GetBody)))
  (Transformation|AddLocalRotation (Variables|Default|GetBody) (Math|Rotator|MakeRotator (.pitch (Variables|Default|GetPlayerRotDelta)) 0.0 0.0) false false)
  (if (< (.z (Math|Vector|GetUpVector (Variables|Default|GetBody))) 0.174)
    (Transformation|SetWorldRotation (Variables|Default|GetBody) (Variables|Default|GetOldRot) false false)
    (if (> (.roll (Variables|/Script/Engine.SceneComponent|GetRelativeRotation (Variables|Default|GetBody))) 0.0)
      (Variables|Default|SetIsUp true)
      (Utilities|FlowControl|DoOnce (not _startdown) :!label _label
        (:Completed
          (Utilities|FlowControl|Sequence
            (:then_0
              _)
            (:then_1
              (goto _label_2 Reset)))))
      (else
        (Variables|Default|SetIsUp false)
        (Utilities|FlowControl|DoOnce _startdown :!label _label_2
          (:Completed
            (Utilities|FlowControl|Sequence
              (:then_0
                _)
              (:then_1
                (goto _label Reset)))))))
    (Audio|PlaySoundatLocation "/Game/SCP/Blueprints/Sounds/LeverFlip.LeverFlip" (Transformation|GetActorLocation))
    (bind _asroom_base_bp (Utilities|Casting|CastToRoomBase_BP (Actor|GetParentActor)))
    (Default|RaiseEvent _asroom_base_bp self (Variables|Default|GetIsUp))))

(event EventSettlingBehavior
  (bind _body (Variables|Default|GetBody))
  (bind _startdown (Variables|Default|GetStartDown))
  (if (> (.roll (Variables|/Script/Engine.SceneComponent|GetRelativeRotation (Variables|Default|GetBody))) 0.0)
    (Variables|Default|SetTargetRot "0, 0,80.000000")
    (bind _alpha (Timeline|Settle PlayFromStart)
      (:Update
        (Transformation|SetRelativeRotation _body (Math|Rotator|Lerp(Rotator) (Variables|/Script/Engine.SceneComponent|GetRelativeRotation _body) (Variables|Default|GetTargetRot) _alpha true) false false))
      (:Finished
        (if (> (.roll (Variables|/Script/Engine.SceneComponent|GetRelativeRotation (Variables|Default|GetBody))) 0.0)
          (Variables|Default|SetIsUp true)
          (Utilities|FlowControl|DoOnce (not _startdown) :!label _label
            (:Completed
              (Utilities|FlowControl|Sequence
                (:then_0
                  _)
                (:then_1
                  (goto _label_2 Reset)))))
          (else
            (Variables|Default|SetIsUp false)
            (Utilities|FlowControl|DoOnce _startdown :!label _label_2
              (:Completed
                (Utilities|FlowControl|Sequence
                  (:then_0
                    _)
                  (:then_1
                    (goto _label Reset)))))))
        (Audio|PlaySoundatLocation "/Game/SCP/Blueprints/Sounds/LeverFlip.LeverFlip" (Transformation|GetActorLocation))
        (bind _asroom_base_bp (Utilities|Casting|CastToRoomBase_BP (Actor|GetParentActor)))
        (Default|RaiseEvent _asroom_base_bp self (Variables|Default|GetIsUp))))
    (else
      (Variables|Default|SetTargetRot "0, 0,-80.000000")
      (Timeline|Settle PlayFromStart))))

(event EventBeginPlay
  (|CallParentFunction)
  (if (Variables|Default|GetStartDown)
    (Transformation|SetRelativeRotation (Variables|Default|GetBody) "0, 0,-80.000000" false false)))

(fn ConstructionScript
  (|CallParentFunction))