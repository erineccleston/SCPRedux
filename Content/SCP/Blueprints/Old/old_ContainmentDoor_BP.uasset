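; Containment door Blueprint that slides a small and a big door panel between their starting positions and end-marker components.
; Open toggles it when DoorEnabled is set, using a FlipFlop to play or reverse one timeline, and StartOpen triggers opening at BeginPlay.
; A DoOnce, reset on timeline finish, limits open or close sounds to one per movement.
; The construction script sets frame visibility from ShowFrame.
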(event Custom|Open
  (if (Variables|Default|GetDoorEnabled)
    (bind _isa (Utilities|FlowControl|FlipFlop)
      (:A
        (bind _alpha (Timeline|Curve Play)
          (:Update
            (Transformation|SetRelativeLocation (Variables|Default|GetSmallDoor) (Math|Vector|Lerp(Vector) (Variables|Default|GetSDStartLoc) (Variables|/Script/Engine.SceneComponent|GetRelativeLocation (Variables|Default|GetSmallDoorEnd)) _alpha) false false)
            (Transformation|SetRelativeLocation (Variables|Default|GetBigDoor) (Math|Vector|Lerp(Vector) (Variables|Default|GetBDStartLoc) (Variables|/Script/Engine.SceneComponent|GetRelativeLocation (Variables|Default|GetBigDoorEnd)) _alpha) false false)
            (Utilities|FlowControl|DoOnce (Variables|Default|GetStartOpen) :!label _label
              (:Completed
                (if _isa
                  (Audio|PlaySoundatLocation (Variables|Default|GetOpenSound) (Transformation|GetActorLocation))
                  (else
                    (Audio|PlaySoundatLocation (Variables|Default|GetCloseSound) (Transformation|GetActorLocation)))))))
          (:Finished
            (goto _label Reset))))
      (:B
        (Timeline|Curve Reverse)))))

(event EventBeginPlay
  (Variables|Default|SetSDStartLoc (Variables|/Script/Engine.SceneComponent|GetRelativeLocation (Variables|Default|GetSmallDoor)))
  (Variables|Default|SetBDStartLoc (Variables|/Script/Engine.SceneComponent|GetRelativeLocation (Variables|Default|GetBigDoor)))
  (if (Variables|Default|GetStartOpen)
    (bind _isa (Utilities|FlowControl|FlipFlop)
      (:A
        (bind _alpha (Timeline|Curve Play)
          (:Update
            (Transformation|SetRelativeLocation (Variables|Default|GetSmallDoor) (Math|Vector|Lerp(Vector) (Variables|Default|GetSDStartLoc) (Variables|/Script/Engine.SceneComponent|GetRelativeLocation (Variables|Default|GetSmallDoorEnd)) _alpha) false false)
            (Transformation|SetRelativeLocation (Variables|Default|GetBigDoor) (Math|Vector|Lerp(Vector) (Variables|Default|GetBDStartLoc) (Variables|/Script/Engine.SceneComponent|GetRelativeLocation (Variables|Default|GetBigDoorEnd)) _alpha) false false)
            (Utilities|FlowControl|DoOnce (Variables|Default|GetStartOpen) :!label _label
              (:Completed
                (if _isa
                  (Audio|PlaySoundatLocation (Variables|Default|GetOpenSound) (Transformation|GetActorLocation))
                  (else
                    (Audio|PlaySoundatLocation (Variables|Default|GetCloseSound) (Transformation|GetActorLocation)))))))
          (:Finished
            (goto _label Reset))))
      (:B
        (Timeline|Curve Reverse)))))

(fn ConstructionScript
  (Rendering|SetVisibility (Variables|Default|GetFrame) (Variables|Default|GetShowFrame) false))