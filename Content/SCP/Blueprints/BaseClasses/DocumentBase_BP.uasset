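; Base Blueprint for collectible SCP document pickups that, when activated, add their type to the player's Documents list and destroy themselves.
; BeginPlay sets the body material from the document type, choosing note, burnt note or a paper fallback.
; Capsule overlap tracks range, while Tick uses WasRecentlyRendered and paired DoOnce gates to add or remove it from the player's InteractablesInRange as it enters or leaves view.
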(event OnComponentBeginOverlap(Capsule)
  (params (OverlappedComponent :type Primitive%20Component%20Object%20Reference) (OtherActor :type Actor%20Object%20Reference) (OtherComp :type Primitive%20Component%20Object%20Reference) (OtherBodyIndex :type Integer) (bFromSweep :type Boolean) (SweepResult :type Hit%20Result%20Structure%20%28by%20ref%29))
  (Utilities|Casting|CastToSCPReduxCharacter_BP OtherActor)
  (Variables|Default|SetInRange true))

(event OnComponentEndOverlap(Capsule)
  (params (OverlappedComponent :type Primitive%20Component%20Object%20Reference) (OtherActor :type Actor%20Object%20Reference) (OtherComp :type Primitive%20Component%20Object%20Reference) (OtherBodyIndex :type Integer))
  (bind _asscpredux_character_bp (Utilities|Casting|CastToSCPReduxCharacter_BP OtherActor))
  (Variables|Default|SetInRange false)
  (Utilities|Array|RemoveItem (Variables|/Game/SCP/Character/SCPReduxCharacter_BP.SCPReduxCharacter_BP_C|GetInteractablesInRange _asscpredux_character_bp) self)
  (Utilities|FlowControl|DoOnce false) ; enters at Reset
)

(event EventBeginPlay
  (bind _material (CallFunction|GetMaterial))
  (Rendering|Material|SetMaterial (Variables|Default|GetBody) 0 _material))

(event EventActivate
  (Utilities|Array|AddUnique (Variables|/Game/SCP/Character/SCPReduxCharacter_BP.SCPReduxCharacter_BP_C|GetDocuments (CallFunction|GetPlayerChar)) (Variables|Default|GetType))
  (Actor|DestroyActor)
  (|CallParentFunction))

(event EventTick
  (params (DeltaSeconds :type Float%20%28single-precision%29))
  (if (Variables|Default|GetInRange)
    (if (Class|Actor|WasRecentlyRendered 0.2)
      (Utilities|FlowControl|DoOnce false :!label _label
        (:Completed
          (Utilities|Array|Add (Variables|/Game/SCP/Character/SCPReduxCharacter_BP.SCPReduxCharacter_BP_C|GetInteractablesInRange (.AsSCPRedux%20Character%20BP (Utilities|Casting|CastToSCPReduxCharacter_BP (Game|Player|GetPlayerPawn 0)))) self)
          (goto _label_2 Reset)))
      (else
        (Utilities|FlowControl|DoOnce false :!label _label_2
          (:Completed
            (Utilities|Array|RemoveItem (Variables|/Game/SCP/Character/SCPReduxCharacter_BP.SCPReduxCharacter_BP_C|GetInteractablesInRange (.AsSCPRedux%20Character%20BP (Utilities|Casting|CastToSCPReduxCharacter_BP (Game|Player|GetPlayerPawn 0)))) self)
            (goto _label Reset)))))))

(fn ConstructionScript
  (|CallParentFunction))

(fn GetMaterial
  (Utilities|FlowControl|Sequence
    (:then_0
      (switch Utilities|FlowControl|Switch|SwitchonEDocuments (Variables|Default|GetType)
        (:doc106_2
          _)
        (:docAC
          (return "/Game/SCP/ItemMeshes/Materials/BurntNote.BurntNote"))
        (:docdan
          _)
        (:docGonzales
          _)
        (:docIR106
          _)
        (:docLl
          _)
        (:docL2
          _)
        (:docL3
          _)
        (:docL4
          (return "/Game/SCP/ItemMeshes/Materials/BurntNote.BurntNote"))
        (:docL5
          (return "/Game/SCP/ItemMeshes/Materials/BurntNote.BurntNote"))
        (:docL6
          (return "/Game/SCP/ItemMeshes/Materials/BurntNote.BurntNote"))
        (:docRAND1
          _)
        (:docRAND2
          _)
        (:f4
          _)
        (:f5
          _)
        (:f6
          _)
        (:bn
          (return "/Game/SCP/ItemMeshes/Materials/BurntNote.BurntNote"))
        (:sn
          _))
      (return "/Game/SCP/ItemMeshes/Materials/Note.Note"))
    (:then_1
      (return "/Game/SCP/ItemMeshes/Materials/Paper.Paper"))))