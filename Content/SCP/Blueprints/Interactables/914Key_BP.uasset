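; SCP-914's key, an interactable that the player turns while grabbing it.
; Grab input rotates the body, with world pitch clamped at zero or above.
; When its up vector points nearly straight down, it raises an event on the parent RoomBase_BP once, until re-armed by ResetRaiseEvent.
; ResetRotation uses a timeline to lerp the body back to its starting rotation along the shortest path.
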(event Custom|ResetRaiseEvent
  (Utilities|FlowControl|DoOnce false) ; enters at Reset
)

(event Custom|ResetRotation
  (Variables|Default|SetCurrentRotation (Transformation|GetWorldRotation (Variables|Default|GetBody)))
  (bind _alpha (Timeline|Reset PlayFromStart)
    (:Update
      (Transformation|SetWorldRotation (Variables|Default|GetBody) (Math|Rotator|Lerp(Rotator) (Variables|Default|GetCurrentRotation) (Variables|Default|GetStartRotation) _alpha true) false false))))

(event EventBeginPlay
  (Variables|Default|SetStartRotation (Transformation|GetWorldRotation (Variables|Default|GetBody))))

(event EventWhileGrabbed
  (bind _playerrotdelta (Variables|Default|GetPlayerRotDelta))
  (bind _body (Variables|Default|GetBody))
  (bind _returnvalue (Transformation|GetWorldRotation _body))
  (Transformation|AddLocalRotation (Variables|Default|GetBody) (Math|Rotator|MakeRotator (.roll _playerrotdelta) (.yaw _playerrotdelta) (.pitch _playerrotdelta)) false false)
  (if (< (.pitch (Transformation|GetWorldRotation (Variables|Default|GetBody))) 0.0)
    (Transformation|SetWorldRotation _body (Math|Rotator|MakeRotator (.roll _returnvalue) 0.0 (.yaw _returnvalue)) false false))
  (if (Math|Vector|Equal(Vector) (Math|Vector|GetUpVector (Variables|Default|GetBody)) "0, 0,-1.000000" 0.05)
    (Utilities|FlowControl|DoOnce false
      (:Completed
        (bind _asroom_base_bp (Utilities|Casting|CastToRoomBase_BP (Actor|GetParentActor)))
        (Default|RaiseEvent _asroom_base_bp self)))))

(fn ConstructionScript
  (|CallParentFunction))