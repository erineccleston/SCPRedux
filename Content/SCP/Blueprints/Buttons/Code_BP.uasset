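; Keypad button that takes a numeric access code from the player and triggers the parent button's activation when it matches.
; Activate moves the player's camera to the keypad and enables input, and digit keys append to a four-character text display with a click sound.
; Enter checks the code and briefly shows a colored granted or denied message.
; Both Tab and Enter return camera control and disable input.
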(event EventChangeDisplay
  (params (IsOpen :type Boolean)))

(event EventActivate
  (Default|TakeCameraControl (CallFunction|GetPlayerChar) (Transformation|GetWorldTransform (Variables|Default|GetCameraTransform)))
  (Input|EnableInput (Game|GetPlayerController 0)))

(event Input|KeyboardEvents|Enter
  (params (Key :type Key%20Structure :default "AnyKey"))
  (bind _textrender (Variables|Default|GetTextRender))
  (bind _textrender_2 (Variables|Default|GetTextRender))
  (:Pressed
    (Default|ReturnCameraControl (CallFunction|GetPlayerChar))
    (Input|DisableInput (Game|GetPlayerController 0))
    (if (Utilities|Enum|Equal(Enum) (Utilities|String|ToString(Text) (Variables|/Script/Engine.TextRenderComponent|GetText (Variables|Default|GetTextRender))) (Variables|Default|GetAccessCode))
      (|CallParentFunction)
      (Rendering|Components|TextRender|SetTextRenderColor _textrender_2 (Math|Color|MakeColor 0 255 0 255))
      (Rendering|Components|TextRender|SetText _textrender_2 (Utilities|Text|MakeLiteralText "ACCESS<br>GRANTED"))
      (else
        (Audio|PlaySound2D (Variables|Default|GetFailSound))
        (Rendering|Components|TextRender|SetTextRenderColor _textrender_2 (Math|Color|MakeColor 0 0 255 255))
        (Rendering|Components|TextRender|SetText _textrender_2 (Utilities|Text|MakeLiteralText "ACCESS<br>DENIED"))))
    (Utilities|FlowControl|Delay 4.0)
    (Rendering|Components|TextRender|SetTextRenderColor _textrender (Math|Color|MakeColor 0 0 0 255))
    (Rendering|Components|TextRender|SetText _textrender (Utilities|Text|MakeLiteralText ""))))

(event Input|KeyboardEvents|AnyKey
  (params (Key :type Key%20Structure :default "AnyKey"))
  (bind _returnvalue (Class|KismetInputLibrary|KeyGetDisplayName Key))
  (bind _textrender (Variables|Default|GetTextRender))
  (bind _returnvalue_2 (Utilities|String|ToString(Text) _returnvalue))
  (bind _returnvalue_3 (Utilities|String|GetCharacterArrayfromString _returnvalue_2))
  (:Pressed
    (switch string _returnvalue_2
      (:Num%200
        _)
      (:Num%201
        _)
      (:Num%202
        _)
      (:Num%203
        _)
      (:Num%204
        _)
      (:Num%205
        _)
      (:Num%206
        _)
      (:Num%207
        _)
      (:Num%208
        _)
      (:Num%209
        _)
      (:0
        _)
      (:1
        _)
      (:2
        _)
      (:3
        _)
      (:4
        _)
      (:5
        _)
      (:6
        _)
      (:7
        _)
      (:8
        _)
      (:9
        _))
    (if (< (Utilities|String|Len (Utilities|String|ToString(Text) (Variables|/Script/Engine.TextRenderComponent|GetText (Variables|Default|GetTextRender)))) 4)
      (Rendering|Components|TextRender|SetText _textrender (Utilities|Text|ToText(String) (Utilities|String|Append (Utilities|String|ToString(Text) (Variables|/Script/Engine.TextRenderComponent|GetText _textrender)) (Utilities|Array|Get(acopy) _returnvalue_3 (- (Utilities|Array|Length _returnvalue_3) 1))))))
    (Audio|PlaySound2D "/Game/SCP/Blueprints/Sounds/Button.Button")))

(event Input|KeyboardEvents|Tab
  (params (Key :type Key%20Structure :default "AnyKey"))
  (:Pressed
    (Default|ReturnCameraControl (CallFunction|GetPlayerChar))
    (Input|DisableInput (Game|GetPlayerController 0))))

(fn ConstructionScript
  (|CallParentFunction)
  (Rendering|Material|SetTextureParameterValue (Variables|Default|GetDynMatInst) "SCPTex" "/Game/SCP/Blueprints/Materials/Textures/KeyPad.KeyPad"))