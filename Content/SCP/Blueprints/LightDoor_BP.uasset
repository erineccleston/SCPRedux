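; LightDoor_BP is a two-panel door that toggles open and closed with sound.
; On BeginPlay it registers itself as Parent of two Button_BP child actors.
; Open alternates playing and reversing a timeline that lerps SmallDoor and BigDoor toward their end-marker component positions.
; A DoOnce, reset when the timeline finishes, plays the open or close sound once per movement based on the FlipFlop state.
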(event Custom|Open
  (bind _isa (Utilities|FlowControl|FlipFlop)
    (:A
      (bind _alpha (Timeline|Curve Play)
        (:Update
          (Transformation|SetRelativeLocation (Variables|Default|GetSmallDoor) (Math|Vector|Lerp(Vector) "4.000000,-8.000000, 0" (Variables|/Script/Engine.SceneComponent|GetRelativeLocation (Variables|Default|GetSmallDoorEnd)) _alpha) false false)
          (Transformation|SetRelativeLocation (Variables|Default|GetBigDoor) (Math|Vector|Lerp(Vector) "-4.000000,8.000000, 0" (Variables|/Script/Engine.SceneComponent|GetRelativeLocation (Variables|Default|GetBigDoorEnd)) _alpha) false false)
          (Utilities|FlowControl|DoOnce false :!label _label
            (:Completed
              (if _isa
                (Audio|PlaySoundatLocation "/Game/SCP/Blueprints/Sounds/DoorOpen.DoorOpen" (Transformation|GetActorLocation))
                (else
                  (Audio|PlaySoundatLocation "/Game/SCP/Blueprints/Sounds/DoorClose.DoorClose" (Transformation|GetActorLocation)))))))
        (:Finished
          (goto _label Reset))))
    (:B
      (Timeline|Curve Reverse))))

(event EventBeginPlay
  (bind _asbutton_bp (Utilities|Casting|CastToButton_BP (Variables|/Script/Engine.ChildActorComponent|GetChildActor (Variables|Default|GetButton1))))
  (Variables|/Game/SCP/Blueprints/Button_BP.Button_BP_C|SetParent _asbutton_bp self)
  (bind _asbutton_bp_2 (Utilities|Casting|CastToButton_BP (Variables|/Script/Engine.ChildActorComponent|GetChildActor (Variables|Default|GetButton2))))
  (Variables|/Game/SCP/Blueprints/Button_BP.Button_BP_C|SetParent _asbutton_bp_2 self))

(fn ConstructionScript)