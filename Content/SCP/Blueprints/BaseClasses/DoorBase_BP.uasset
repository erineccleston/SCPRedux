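; Base Blueprint for SCP two-panel doors that slide open and closed, with optional start-open, timed and zone-transition behavior.
; A FlipFlop drives a timeline that lerps both panels to end markers and plays sounds, while a DoOnce blocks repeat Open calls mid-cycle.
; On finish it updates button displays; timed doors sound a siren, then close automatically.
; SetAsParent links child-actor buttons to a door and sets its clearance level.
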(event Custom|Open
  (bind _returnvalue (Transformation|GetActorLocation))
  (Utilities|FlowControl|DoOnce false
    (:Completed
      (bind _isa (Utilities|FlowControl|FlipFlop)
        (:A
          (bind _alpha (Timeline|Curve Play)
            (:Update
              (Transformation|SetRelativeLocation (Variables|Default|GetDoor2) (Math|Vector|Lerp(Vector) (Variables|Default|GetDoor2Start) (Variables|/Script/Engine.SceneComponent|GetRelativeLocation (Variables|Default|GetDoor2End)) _alpha) false false)
              (Transformation|SetRelativeLocation (Variables|Default|GetDoor1) (Math|Vector|Lerp(Vector) (Variables|Default|GetDoor1Start) (Variables|/Script/Engine.SceneComponent|GetRelativeLocation (Variables|Default|GetDoor1End)) _alpha) false false)
              (Utilities|FlowControl|DoOnce (Variables|Default|GetStartOpen) :!label _label
                (:Completed
                  (if _isa
                    (Audio|PlaySoundatLocation (Variables|Default|GetOpenSound) _returnvalue)
                    (else
                      (Audio|PlaySoundatLocation (Variables|Default|GetCloseSound) _returnvalue "0, 0, 0" 1.0 1.0 0.0)))
                  (if (Variables|Default|GetIsZoneTransition)
                    (Audio|PlaySoundatLocation "/Game/SCP/Blueprints/Sounds/DoorCheckpoint.DoorCheckpoint" _returnvalue)))))
            (:Finished
              (Utilities|FlowControl|Sequence
                (:then_0
                  (goto _label Reset))
                (:then_1
                  (CallFunction|NotifyButtons _isa)
                  (if (Variables|Default|GetIsTimed)
                    (Utilities|FlowControl|FlipFlop
                      (:A
                        (Utilities|FlowControl|Delay 3.5)
                        (Audio|PlaySoundatLocation "/Game/SCP/Blueprints/Sounds/LockroomSiren.LockroomSiren" (Transformation|GetActorLocation))
                        (Utilities|FlowControl|Delay 1.5)
                        (CallFunction|Reverse))
                      (:B
                        (CallFunction|Reset :!label _label_2)))
                    (else
                      (goto _label_2))))))))
        (:B
          (Timeline|Curve Reverse))))))

(event Custom|Reset
  (bind _returnvalue (Transformation|GetActorLocation))
  (Utilities|FlowControl|DoOnce false) ; enters at Reset
)

(event Custom|Reverse
  (bind _returnvalue (Transformation|GetActorLocation))
  (bind _isa (Utilities|FlowControl|FlipFlop)
    (:A
      (bind _alpha (Timeline|Curve Play)
        (:Update
          (Transformation|SetRelativeLocation (Variables|Default|GetDoor2) (Math|Vector|Lerp(Vector) (Variables|Default|GetDoor2Start) (Variables|/Script/Engine.SceneComponent|GetRelativeLocation (Variables|Default|GetDoor2End)) _alpha) false false)
          (Transformation|SetRelativeLocation (Variables|Default|GetDoor1) (Math|Vector|Lerp(Vector) (Variables|Default|GetDoor1Start) (Variables|/Script/Engine.SceneComponent|GetRelativeLocation (Variables|Default|GetDoor1End)) _alpha) false false)
          (Utilities|FlowControl|DoOnce (Variables|Default|GetStartOpen) :!label _label
            (:Completed
              (if _isa
                (Audio|PlaySoundatLocation (Variables|Default|GetOpenSound) _returnvalue)
                (else
                  (Audio|PlaySoundatLocation (Variables|Default|GetCloseSound) _returnvalue "0, 0, 0" 1.0 1.0 0.0)))
              (if (Variables|Default|GetIsZoneTransition)
                (Audio|PlaySoundatLocation "/Game/SCP/Blueprints/Sounds/DoorCheckpoint.DoorCheckpoint" _returnvalue)))))
        (:Finished
          (Utilities|FlowControl|Sequence
            (:then_0
              (goto _label Reset))
            (:then_1
              (CallFunction|NotifyButtons _isa)
              (if (Variables|Default|GetIsTimed)
                (Utilities|FlowControl|FlipFlop
                  (:A
                    (Utilities|FlowControl|Delay 3.5)
                    (Audio|PlaySoundatLocation "/Game/SCP/Blueprints/Sounds/LockroomSiren.LockroomSiren" (Transformation|GetActorLocation))
                    (Utilities|FlowControl|Delay 1.5)
                    (CallFunction|Reverse))
                  (:B
                    (CallFunction|Reset :!label _label_2)))
                (else
                  (goto _label_2))))))))
    (:B
      (Timeline|Curve Reverse))))

(event EventBeginPlay
  (Variables|Default|SetDoor2Start (Variables|/Script/Engine.SceneComponent|GetRelativeLocation (Variables|Default|GetDoor2)))
  (Variables|Default|SetDoor1Start (Variables|/Script/Engine.SceneComponent|GetRelativeLocation (Variables|Default|GetDoor1)))
  (Components|Timeline|SetPlayRate (Variables|Default|GetCurve) (Variables|Default|GetPlayRate))
  (if (Variables|Default|GetStartOpen)
    (CallFunction|Reverse)))

(fn ConstructionScript
  (Variables|Default|SetIsOpen (Variables|Default|GetStartOpen)))

(fn SetasParent
  (params (Door :type Child%20Actor%20Component%20Object%20Reference) (Button1 :type Child%20Actor%20Component%20Object%20Reference) (Button2 :type Child%20Actor%20Component%20Object%20Reference) (ClearanceLevel :type Integer))
  (bind _asdoor_base_bp (Utilities|Casting|CastToDoorBase_BP (Variables|/Script/Engine.ChildActorComponent|GetChildActor Door)))
  (bind _output_get (LocalVariables|SetDoorRef _asdoor_base_bp))
  (Variables|DoorBase_BP_C|SetClearanceLevel _output_get ClearanceLevel)
  (bind _asbutton_base_bp (Utilities|Casting|CastToButtonBase_BP (Variables|/Script/Engine.ChildActorComponent|GetChildActor Button1)))
  (Variables|/Game/SCP/Blueprints/BaseClasses/ButtonBase_BP.ButtonBase_BP_C|SetParentDoor _asbutton_base_bp (LocalVariables|GetDoorRef))
  (bind _asbutton_base_bp_2 (Utilities|Casting|CastToButtonBase_BP (Variables|/Script/Engine.ChildActorComponent|GetChildActor Button2)))
  (Variables|/Game/SCP/Blueprints/BaseClasses/ButtonBase_BP.ButtonBase_BP_C|SetParentDoor _asbutton_base_bp_2 (LocalVariables|GetDoorRef)))

(fn NotifyButtons
  (params (IsOpen :type Boolean))
  (for _array_element (Variables|Default|GetChildButtons)
    (Default|ChangeDisplay _array_element IsOpen)))