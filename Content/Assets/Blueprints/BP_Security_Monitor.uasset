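; BP_Security_Monitor is a monitor that shows a security camera's scene capture on its screen.
; The construction script creates a dynamic material instance on the monitor mesh's screen slot.
; On BeginPlay it sets the Noise parameter to zero, noted as a workaround for the screen not updating, then activates CameraBlueprint's capture and applies the returned texture.
; Its own SceneCaptureActivation function is an empty stub.
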(event EventBeginPlay
  (Utilities|FlowControl|Sequence
    (:then_0
      ;[1 1 1] For some reason this has to happen or the screen won't update to have the camera texture.
      (Rendering|Material|SetScalarParameterValue (Variables|Default|GetMonitor%20material) "Noise" 0.0 :!class /Script/Engine.MaterialInstanceDynamic) ; Briefly flash a noise effect on the monitor screen
    )
    (:then_1
      (bind _capture_texture (Class|BPISecurityAlarmInterface|SceneCaptureActivation(Message) (Variables|Default|GetCamera%20Blueprint) true)) ; Turn on scene capture for the next camera in the sequence
      (Rendering|Material|SetTextureParameterValue (Variables|Default|GetMonitor%20material) "Screen Texture" _capture_texture) ; Get the scene texture used by the camera and apply it to the monitor material
    )))

(fn ConstructionScript
  (bind _returnvalue (Rendering|Material|CreateDynamicMaterialInstance (Variables|Default|GetMonitorMesh) 1 0 :!class /Script/Engine.PrimitiveComponent))
  (Variables|Default|SetMonitor%20material _returnvalue))

(fn SceneCaptureActivation
  (params (Activation :type Boolean))
  (return 0))