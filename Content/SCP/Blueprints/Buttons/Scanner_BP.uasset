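; Scanner_BP is a palm/DNA scanner button for the SCP game that gates its parent activation behind a required hand item.
; On Activate, it compares the player character's ActiveItem to the CorrectHand of the first entry in Parents.
; A match runs the parent Activate and then sets ActiveItem to a fixed enum value.
; A mismatch plays a fail sound and queues an access-denied message.
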(event EventBeginPlay)

(event Collision|EventActorBeginOverlap
  (params (OtherActor :type Actor%20Object%20Reference)))

(event EventTick
  (params (DeltaSeconds :type Float%20%28single-precision%29)))

(event EventActivate
  (bind _asscpredux_character_bp (Utilities|Casting|CastToSCPReduxCharacter_BP (Game|Player|GetPlayerPawn 0)))
  (if (Utilities|Enum|Equal(Enum) (Variables|/Game/SCP/Character/SCPReduxCharacter_BP.SCPReduxCharacter_BP_C|GetActiveItem _asscpredux_character_bp) (Variables|/Game/SCP/Blueprints/BaseClasses/DoorBase_BP.DoorBase_BP_C|GetCorrectHand (Utilities|Array|Get(acopy) (Variables|Default|GetParents))))
    (|CallParentFunction)
    (bind _asscpredux_character_bp_2 (Utilities|Casting|CastToSCPReduxCharacter_BP (Game|Player|GetPlayerPawn 0)))
    (Variables|/Game/SCP/Character/SCPReduxCharacter_BP.SCPReduxCharacter_BP_C|SetActiveItem _asscpredux_character_bp_2 "NewEnumerator59")
    (else
      (Audio|PlaySoundatLocation (Variables|Default|GetFailSound) (Transformation|GetActorLocation))
      (Default|QueueMessage _asscpredux_character_bp "You placed your palm onto the scanner. The scanner reads: \"DNA does not match known sample. Access denied.\""))))

(fn ConstructionScript
  (|CallParentFunction))