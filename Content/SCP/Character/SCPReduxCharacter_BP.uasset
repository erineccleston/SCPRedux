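; Player character for an SCP game, handling health, sprint stamina, blinking and death.
; BeginPlay creates its HUD widgets, and Tick applies bleed damage, drains or regenerates stamina with an exhaustion cooldown, and drains blink until a forced blink.
; Sprint state swaps a movement struct that drives headbob shake and Delay-paced footsteps.
; DamageBase_BP damage types supply the death message Kill shows before detaching the controller.
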(event Custom|SimulateBlink
  (bind _blinkoverlay (Variables|Widgets|GetBlinkOverlay))
  (bind _blinkoverlay_2 (Variables|Widgets|GetBlinkOverlay))
  (UserInterface|Animation|PlayAnimation _blinkoverlay_2 (Variables|/Game/SCP/HUD/BlinkOverlay.BlinkOverlay_C|GetFade%20In _blinkoverlay_2) 0.0 1 "Forward" 1.0)
  (Variables|Blink|SetEyesClosed true)
  (Utilities|FlowControl|Delay 0.2)
  (UserInterface|Animation|PlayAnimation _blinkoverlay (Variables|/Game/SCP/HUD/BlinkOverlay.BlinkOverlay_C|GetFade%20In _blinkoverlay) 0.0 1 "Reverse" 1.0)
  (Variables|Blink|SetEyesClosed false)
  (Variables|Blink|SetBlinkValue (Variables|Blink|GetMaxBlink)))

(event Custom|Queue%20Message
  (params (Message :type String))
  (bind _textpopup (Variables|Widgets|GetTextPopup))
  (Variables|Widgets|SetMessage Message)
  (UserInterface|Animation|PlayAnimation _textpopup (Variables|/Game/SCP/HUD/TextPopup.TextPopup_C|GetFade _textpopup) 0.0 1 "Forward" 1.0))

(event Custom|Kill
  (bind _deathmenu (Variables|Widgets|GetDeathMenu))
  (Widget|SetVisibility (Variables|Widgets|GetBlinkOverlay) "Hidden")
  (Widget|SetVisibility _deathmenu "Visible")
  (Variables|/Game/SCP/Menu/DeathMenu.DeathMenu_C|SetLastDeathMessage _deathmenu (Variables|Health|GetDeathMessage))
  (Variables|Stamina|SetDrainStamina false)
  (Class|Pawn|DetachfromControllerPendingDestroy))

(event EventBeginPlay
  (Utilities|FlowControl|Sequence
    (:then_0
      (bind _returnvalue (UserInterface|CreateWidget "/Game/SCP/HUD/BlinkOverlay.BlinkOverlay_C"))
      (bind _output_get (Variables|Widgets|SetBlinkOverlay _returnvalue))
      (UserInterface|Viewport|AddtoViewport _output_get 0)
      (bind _returnvalue_2 (UserInterface|CreateWidget "/Game/SCP/HUD/BlinkStaminaMeters.BlinkStaminaMeters_C"))
      (bind _output_get_2 (Variables|Widgets|SetBlinkStaminaMeters _returnvalue_2))
      (UserInterface|Viewport|AddtoViewport _output_get_2 0)
      (bind _returnvalue_3 (UserInterface|CreateWidget "/Game/SCP/HUD/InteractIcon.InteractIcon_C"))
      (bind _output_get_3 (Variables|Widgets|SetInteractIcon _returnvalue_3))
      (UserInterface|Viewport|AddtoViewport _output_get_3 0)
      (bind _returnvalue_4 (UserInterface|CreateWidget "/Game/SCP/HUD/TextPopup.TextPopup_C"))
      (bind _output_get_4 (Variables|Widgets|SetTextPopup _returnvalue_4))
      (UserInterface|Viewport|AddtoViewport _output_get_4 0)
      (bind _returnvalue_5 (UserInterface|CreateWidget "/Game/SCP/Menu/DeathMenu.DeathMenu_C"))
      (bind _output_get_5 (Variables|Widgets|SetDeathMenu _returnvalue_5))
      (UserInterface|Viewport|AddtoViewport _output_get_5 0))
    (:then_1
      (CallFunction|StopSprinting))))

(event EventTick
  (params (DeltaSeconds :type Float%20%28single-precision%29))
  (Variables|Misc|SetDeltaSeconds DeltaSeconds)
  (CallFunction|ChangeHealth)
  (CallFunction|ChangeStamina)
  (CallFunction|DrainBlink))

(event Game|Damage|EventAnyDamage
  (params (Damage :type Float%20%28single-precision%29) (DamageType :type Damage%20Type%20Object%20Reference) (InstigatedBy :type Controller%20Object%20Reference) (DamageCauser :type Actor%20Object%20Reference))
  (Variables|Health|SetHealthValue (- (Variables|Health|GetHealthValue) Damage))
  (bind _asdamage_base_bp (Utilities|Casting|CastToDamageBase_BP DamageType))
  (bind _death_message (Default|GetDeathMessage _asdamage_base_bp))
  (Variables|Health|SetDeathMessage _death_message))

(event Input|ActionEvents|InputActionSprint
  (params (Key :type Key%20Structure :default "AnyKey"))
  (:Pressed
    (if (> (Variables|Stamina|GetStaminaValue) 0.0)
      (CallFunction|StartSprinting)))
  (:Released
    (CallFunction|StopSprinting)))

(event Input|ActionEvents|InputActionBlink
  (params (Key :type Key%20Structure :default "AnyKey"))
  (bind _blinkoverlay (Variables|Widgets|GetBlinkOverlay))
  (bind _blinkoverlay_2 (Variables|Widgets|GetBlinkOverlay))
  (:Pressed
    (UserInterface|Animation|PlayAnimation _blinkoverlay_2 (Variables|/Game/SCP/HUD/BlinkOverlay.BlinkOverlay_C|GetFade%20In _blinkoverlay_2) 0.0 1 "Forward" 1.0)
    (Variables|Blink|SetEyesClosed true)
    (Variables|Blink|SetBlinkValue 0.0))
  (:Released
    (Utilities|FlowControl|Delay 0.2)
    (UserInterface|Animation|PlayAnimation _blinkoverlay (Variables|/Game/SCP/HUD/BlinkOverlay.BlinkOverlay_C|GetFade%20In _blinkoverlay) 0.0 1 "Reverse" 1.0)
    (Variables|Blink|SetEyesClosed false)
    (Variables|Blink|SetBlinkValue (Variables|Blink|GetMaxBlink))))

(event Input|ActionEvents|InputActionInventory
  (params (Key :type Key%20Structure :default "AnyKey")))

(event Input|AxisEvents|InputAxisMoveForward
  (params (AxisValue :type Float%20%28single-precision%29))
  (bind _movpar (Variables|Misc|GetMovPar))
  (if (!= AxisValue 0.0)
    (Pawn|Input|AddMovementInput (Transformation|GetActorForwardVector) AxisValue false)
    (if (Math|Vector|NotEqual(Vector) (Transformation|GetVelocity) "0, 0, 0" 0.0001)
      (Class|PlayerController|ClientPlayCameraShake (Game|GetPlayerController 0) (.headbob _movpar) 1.0 "CameraLocal" "0, 0, 0")
      (Utilities|FlowControl|Delay (.delay _movpar))
      (Audio|PlaySoundatLocation (.sound _movpar) (Transformation|GetActorLocation)))))

(event Input|AxisEvents|InputAxisMoveRight
  (params (AxisValue :type Float%20%28single-precision%29))
  (bind _movpar (Variables|Misc|GetMovPar))
  (if (!= AxisValue 0.0)
    (Pawn|Input|AddMovementInput (Transformation|GetActorRightVector) AxisValue false)
    (if (Math|Vector|NotEqual(Vector) (Transformation|GetVelocity) "0, 0, 0" 0.0001)
      (Class|PlayerController|ClientPlayCameraShake (Game|GetPlayerController 0) (.headbob _movpar) 1.0 "CameraLocal" "0, 0, 0")
      (Utilities|FlowControl|Delay (.delay _movpar))
      (Audio|PlaySoundatLocation (.sound _movpar) (Transformation|GetActorLocation)))))

(fn ConstructionScript)

(fn DrainBlink
  (if (not (Variables|Blink|GetEyesClosed))
    (if (< (Variables|Blink|GetBlinkValue) 0.0)
      (CallFunction|SimulateBlink)
      (else
        (Variables|Blink|SetBlinkValue (- (Variables|Blink|GetBlinkValue) (* (Variables|Misc|GetDeltaSeconds) (Variables|Blink|GetBlinkDrainRate))))))))

(fn ChangeStamina
  (if (and (Math|Vector|NotEqual(Vector) (Transformation|GetVelocity) "0, 0, 0" 0.0001) (Variables|Stamina|GetDrainStamina))
    (if (> (Variables|Stamina|GetStaminaValue) 0.0)
      (bind _output_get (Variables|Stamina|SetStaminaValue (- (Variables|Stamina|GetStaminaValue) (* (Variables|Misc|GetDeltaSeconds) (Variables|Stamina|GetStaminaDrainRate)))))
      (if (<= _output_get 0.0)
        (CallFunction|StopSprinting)
        (Variables|Stamina|SetLastSprintTime (+ (Utilities|Time|GetGameTimeinSeconds) (Variables|Stamina|GetStaminaCooldown)))
        (Audio|PlaySound2D "/Game/SCP/Character/Sounds/breath0.breath0")))
    (elif (and (< (Variables|Stamina|GetLastSprintTime) (Utilities|Time|GetGameTimeinSeconds)) (< (Variables|Stamina|GetStaminaValue) (Variables|Stamina|GetMaxStamina)))
      (Variables|Stamina|SetStaminaValue (+ (Variables|Stamina|GetStaminaValue) (* (Variables|Misc|GetDeltaSeconds) (Variables|Stamina|GetStaminaRegenRate)))))))

(fn StartSprinting
  (Variables|/Script/Engine.CharacterMovementComponent|SetMaxWalkSpeed (Variables|Character|GetCharacterMovement) (Variables|Movement|GetSprintSpeed))
  (Variables|Stamina|SetDrainStamina true)
  (Variables|Misc|SetMovPar (Utilities|Struct|MakeMovementParameters 0.55 "/Game/SCP/Character/Sounds/Run.Run" "/Game/SCP/Character/HeadbobRun.HeadbobRun_C" 7e+02)))

(fn StopSprinting
  (Variables|/Script/Engine.CharacterMovementComponent|SetMaxWalkSpeed (Variables|Character|GetCharacterMovement) (Variables|Movement|GetWalkSpeed))
  (Variables|Stamina|SetDrainStamina false)
  (Variables|Misc|SetMovPar (Utilities|Struct|MakeMovementParameters 0.75 "/Game/SCP/Character/Sounds/Step.Step" "/Game/SCP/Character/HeadbobWalk.HeadbobWalk_C" 3e+02)))

(fn ChangeHealth
  (if (> (Variables|Health|GetHealthValue) 0.0)
    (if (> (Variables|Health|GetBleedRate) 0.0)
      (Game|Damage|ApplyDamage self (Variables|Health|GetBleedRate) 0 0))
    (else
      (CallFunction|Kill))))