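; Base Blueprint for collectible documents in the SCP game, which adds its document type to the player's collection and destroys itself when activated.
; On BeginPlay it picks a note, burnt note or paper material based on its type.
; Capsule overlap and a recently-rendered check on Tick control its entry in the player's interactables list, with DoOnce gates limiting repeated adds and removes.
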(event OnComponentBeginOverlap(Capsule)
  (params (OverlappedComponent :type Primitive%20Component%20Object%20Reference) (OtherActor :type Actor%20Object%20Reference) (OtherComp :type Primitive%20Component%20Object%20Reference) (OtherBodyIndex :type Integer) (bFromSweep :type Boolean) (SweepResult :type Hit%20Result%20Structure%20%28by%20ref%29))
  (Utilities|Casting|CastToSCPReduxCharacter_BP OtherActor)
  (Variables|Default|SetInRange true))

(event OnComponentEndOverlap(Capsule)
  (params (OverlappedComponent :type Primitive%20Component%20Object%20Reference) (OtherActor :type Actor%20Object%20Reference) (OtherComp :type Primitive%20Component%20Object%20Reference) (OtherBodyIndex :type Integer))
  (bind _asscpredux_character_bp (Utilities|Casting|CastToSCPReduxCharacter_BP OtherActor))
  (Variables|Default|SetInRange false)
  (Utilities|Array|RemoveItem (Variables|/Game/SCP/Character/SCPReduxCharacter_BP.SCPReduxCharacter_BP_C|GetInteractablesInRange _asscpredux_character_bp) self)
  (Utilities|FlowControl|DoOnce false) ; enters at Reset
)

(event EventBeginPlay
  (bind _material (CallFunction|GetMaterial))
  (Rendering|Material|SetMaterial (Variables|Default|GetBody) 0 _material))

(event EventActivate
  (Utilities|Array|AddUnique (Variables|/Game/SCP/Character/SCPReduxCharacter_BP.SCPReduxCharacter_BP_C|GetDocuments (CallFunction|GetPlayerChar)) (Variables|Default|GetType))
  (Actor|DestroyActor)
  (|CallParentFunction))

(event EventTick
  (params (DeltaSeconds :type Float%20%28single-precision%29))
  (if (Variables|Default|GetInRange)
    (if (Class|Actor|WasRecentlyRendered 0.2)
      (Utilities|FlowControl|DoOnce false :!label _label
        (:Completed
          (Utilities|Array|Add (Variables|/Game/SCP/Character/SCPReduxCharacter_BP.SCPReduxCharacter_BP_C|GetInteractablesInRange (.AsSCPRedux%20Character%20BP (Utilities|Casting|CastToSCPReduxCharacter_BP (Game|Player|GetPlayerPawn 0)))) self)
          (goto _label_2 Reset)))
      (else
        (Utilities|FlowControl|DoOnce false :!label _label_2
          (:Completed
            (Utilities|Array|RemoveItem (Variables|/Game/SCP/Character/SCPReduxCharacter_BP.SCPReduxCharacter_BP_C|GetInteractablesInRange (.AsSCPRedux%20Character%20BP (Utilities|Casting|CastToSCPReduxCharacter_BP (Game|Player|GetPlayerPawn 0)))) self)
            (goto _label Reset)))))))

(fn ConstructionScript
  (|CallParentFunction))

(fn GetMaterial
  (Utilities|FlowControl|Sequence
    (:then_0
      (switch Utilities|FlowControl|Switch|SwitchonDocs_Enum (Variables|Default|GetType)
        (:NewEnumerator11
          _)
        (:NewEnumerator31
          (return "/Game/SCP/ItemMeshes/Materials/BurntNote.BurntNote"))
        (:NewEnumerator32
          _)
        (:NewEnumerator33
          _)
        (:NewEnumerator34
          _)
        (:NewEnumerator35
          _)
        (:NewEnumerator36
          _)
        (:NewEnumerator37
          _)
        (:NewEnumerator38
          (return "/Game/SCP/ItemMeshes/Materials/BurntNote.BurntNote"))
        (:NewEnumerator39
          (return "/Game/SCP/ItemMeshes/Materials/BurntNote.BurntNote"))
        (:NewEnumerator40
          (return "/Game/SCP/ItemMeshes/Materials/BurntNote.BurntNote"))
        (:NewEnumerator46
          _)
        (:NewEnumerator47
          _))
      (return "/Game/SCP/ItemMeshes/Materials/Note.Note"))
    (:then_1
      (return "/Game/SCP/ItemMeshes/Materials/Paper.Paper"))))