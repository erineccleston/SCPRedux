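; A legacy button Blueprint that opens the door it is attached to and gives success or failure feedback.
; On activation it casts its parent actor to DoorBase_BP, copies the door's fail message and calls Open.
; An enabled door sets the success sound; a disabled or missing door sets the fail sound and queues the message on the player character.
; The parent Activate then runs.
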(event EventActivate
  (bind _asdoor_base_bp (Utilities|Casting|CastToDoorBase_BP (Actor|GetParentActor))
    (:then
      (Variables|Default|SetFailMessage (Variables|/Game/SCP/Blueprints/BaseClasses/DoorBase_BP.DoorBase_BP_C|GetFailMessage _asdoor_base_bp))
      (Default|Open _asdoor_base_bp)
      (if (Variables|/Game/SCP/Blueprints/BaseClasses/DoorBase_BP.DoorBase_BP_C|GetDoorEnabled _asdoor_base_bp)
        (Variables|Default|SetInteractSound (Variables|Default|GetSuccessSound))
        (else
          (Variables|Default|SetInteractSound (Variables|Default|GetFailSound) :!label _label)
          (bind _asscpredux_character_bp (Utilities|Casting|CastToSCPReduxCharacter_BP (Game|Player|GetPlayerPawn 0)))
          (Default|QueueMessage _asscpredux_character_bp (Variables|Default|GetFailMessage)))))
    (:CastFailed
      (goto _label)))
  (|CallParentFunction))

(fn ConstructionScript)