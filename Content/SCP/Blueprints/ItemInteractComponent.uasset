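; Actor component that makes its owning item interactable when the SCP player character is in range and the item is on screen.
; Owner capsule overlaps set InRange, and Tick combines it with a recently-rendered check.
; While both hold, the player's hand icon follows the item's projected position, clamped within screen margins.
; Paired DoOnce gates toggle owner input and update the player's ItemsInRange count on state changes.
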(event Custom|OnComponentBeginOverlap_Event_0
  (params (OverlappedComponent :type Primitive%20Component%20Object%20Reference) (OtherActor :type Actor%20Object%20Reference) (OtherComp :type Primitive%20Component%20Object%20Reference) (OtherBodyIndex :type Integer) (bFromSweep :type Boolean) (SweepResult :type Hit%20Result%20Structure%20%28by%20ref%29))
  (Utilities|Casting|CastToSCPReduxCharacter_BP OtherActor)
  (Variables|Default|SetInRange true))

(event Custom|OnComponentEndOverlap_Event_0
  (params (OverlappedComponent :type Primitive%20Component%20Object%20Reference) (OtherActor :type Actor%20Object%20Reference) (OtherComp :type Primitive%20Component%20Object%20Reference) (OtherBodyIndex :type Integer))
  (Utilities|Casting|CastToSCPReduxCharacter_BP OtherActor)
  (Variables|Default|SetInRange false))

(event EventBeginPlay
  (bind _returnvalue (Components|GetOwner))
  (bind _returnvalue_2 (Actor|GetComponentbyClass _returnvalue "/Script/Engine.CapsuleComponent"))
  (Collision|AssignOnComponentBeginOverlap _returnvalue_2 (delegate Custom|OnComponentBeginOverlap_Event_0))
  (Collision|AssignOnComponentEndOverlap _returnvalue_2 (delegate Custom|OnComponentEndOverlap_Event_0))
  (bind _asscpredux_character_bp (Utilities|Casting|CastToSCPReduxCharacter_BP (Game|Player|GetPlayerPawn 0)))
  (Variables|Default|SetPlayerChar _asscpredux_character_bp)
  (Variables|Default|SetIconRef (Variables|/Game/SCP/Character/SCPReduxCharacter_BP.SCPReduxCharacter_BP_C|GetInteractIcon _asscpredux_character_bp)))

(event EventTick
  (params (DeltaSeconds :type Float%20%28single-precision%29))
  (if (and (Class|Actor|WasRecentlyRendered (Components|GetOwner) 0.2) (Variables|Default|GetInRange))
    (|MoveIcon
      (:NewParam
        (Utilities|FlowControl|DoOnce false :!label _label
          (:Completed
            (Input|EnableInput (Components|GetOwner) (Game|GetPlayerController 0))
            (Variables|/Game/SCP/HUD/InteractIcon.InteractIcon_C|SetImage (Variables|Default|GetIconRef) "/Game/SCP/HUD/Textures/handsymbol2.handsymbol2")
            (Math|Integer|IncrementInt (Variables|/Game/SCP/Character/SCPReduxCharacter_BP.SCPReduxCharacter_BP_C|GetItemsInRange (Variables|Default|GetPlayerChar))
              (:%20%20
                (goto _label_2 Reset)))))))
    (else
      (Utilities|FlowControl|DoOnce false :!label _label_2
        (:Completed
          (Input|DisableInput (Components|GetOwner) (Game|GetPlayerController 0))
          (Math|Integer|DecrementInt (Variables|/Game/SCP/Character/SCPReduxCharacter_BP.SCPReduxCharacter_BP_C|GetItemsInRange (Variables|Default|GetPlayerChar))
            (:%20%20
              (goto _label Reset))))))))