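; Base pickup item that goes into the player's inventory when activated, or queues a message if there is no room.
; Its Type looks up attributes that set mesh, scale and pickup sound, applied from the construction script.
; Activation writes Type into the first slot holding a placeholder value and destroys the actor.
; Capsule overlap and a recently-rendered check on Tick, gated by paired DoOnce nodes, manage its entry in the player's InteractablesInRange.
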(event OnComponentBeginOverlap(Capsule)
  (params (OverlappedComponent :type Primitive%20Component%20Object%20Reference) (OtherActor :type Actor%20Object%20Reference) (OtherComp :type Primitive%20Component%20Object%20Reference) (OtherBodyIndex :type Integer) (bFromSweep :type Boolean) (SweepResult :type Hit%20Result%20Structure%20%28by%20ref%29))
  (Utilities|Casting|CastToSCPReduxCharacter_BP OtherActor)
  (Variables|Default|SetInRange true))

(event OnComponentEndOverlap(Capsule)
  (params (OverlappedComponent :type Primitive%20Component%20Object%20Reference) (OtherActor :type Actor%20Object%20Reference) (OtherComp :type Primitive%20Component%20Object%20Reference) (OtherBodyIndex :type Integer))
  (bind _asscpredux_character_bp (Utilities|Casting|CastToSCPReduxCharacter_BP OtherActor))
  (Variables|Default|SetInRange false)
  (Utilities|Array|RemoveItem (Variables|/Game/SCP/Character/SCPReduxCharacter_BP.SCPReduxCharacter_BP_C|GetInteractablesInRange _asscpredux_character_bp) self))

(event Custom|SetType
  (params (Type :type Items_Enum%20Enum))
  (bind _body (Variables|Default|GetBody))
  (bind _output_get (Variables|Default|SetType Type))
  (bind _attributes (CallFunction|GetAttributes _output_get))
  (bind _output_get_2 (Variables|Default|SetAttributes _attributes))
  (Components|StaticMesh|SetStaticMesh _body (.mesh _output_get_2))
  (Transformation|SetRelativeScale3D _body (Math|Vector|MakeVector (.uniformscale _output_get_2) (.uniformscale _output_get_2) (.uniformscale _output_get_2)))
  (Variables|Default|SetInteractSound (.pickupsound _output_get_2)))

(event EventActivate
  (bind _asscpredux_character_bp (Utilities|Casting|CastToSCPReduxCharacter_BP (Game|Player|GetPlayerPawn 0)))
  (if (>= (Utilities|Array|FindItem (Variables|/Game/SCP/Character/SCPReduxCharacter_BP.SCPReduxCharacter_BP_C|GetInventory _asscpredux_character_bp) "NewEnumerator59") 0)
    (Utilities|Array|SetArrayElem (Variables|/Game/SCP/Character/SCPReduxCharacter_BP.SCPReduxCharacter_BP_C|GetInventory _asscpredux_character_bp) (Utilities|Array|FindItem (Variables|/Game/SCP/Character/SCPReduxCharacter_BP.SCPReduxCharacter_BP_C|GetInventory _asscpredux_character_bp) "NewEnumerator59") (Variables|Default|GetType))
    (Actor|DestroyActor)
    (Math|Integer|DecrementInt (Variables|/Game/SCP/Character/SCPReduxCharacter_BP.SCPReduxCharacter_BP_C|GetItemsInRange _asscpredux_character_bp)
      (:%20%20
        (|CallParentFunction)))
    (else
      (Default|QueueMessage _asscpredux_character_bp "You cannot carry any more items."))))

(event EventTick
  (params (DeltaSeconds :type Float%20%28single-precision%29))
  (if (Variables|Default|GetInRange)
    (if (Class|Actor|WasRecentlyRendered 0.2)
      (Utilities|FlowControl|DoOnce false :!label _label
        (:Completed
          (Utilities|Array|Add (Variables|/Game/SCP/Character/SCPReduxCharacter_BP.SCPReduxCharacter_BP_C|GetInteractablesInRange (.AsSCPRedux%20Character%20BP (Utilities|Casting|CastToSCPReduxCharacter_BP (Game|Player|GetPlayerPawn 0)))) self)
          (goto _label_2 Reset)))
      (else
        (Utilities|FlowControl|DoOnce false :!label _label_2
          (:Completed
            (Utilities|Array|RemoveItem (Variables|/Game/SCP/Character/SCPReduxCharacter_BP.SCPReduxCharacter_BP_C|GetInteractablesInRange (.AsSCPRedux%20Character%20BP (Utilities|Casting|CastToSCPReduxCharacter_BP (Game|Player|GetPlayerPawn 0)))) self)
            (goto _label Reset)))))))

(fn ConstructionScript
  (|CallParentFunction)
  (CallFunction|SetType (Variables|Default|GetType)))