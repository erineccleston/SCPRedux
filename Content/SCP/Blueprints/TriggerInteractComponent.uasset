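; Actor component that makes its owner a proximity interactable, showing a hand icon while the SCP player character overlaps the owner's capsule.
; Capsule overlap begin and end toggle input on the owner and show or hide the character's InteractIcon widget.
; While the icon is shown, Tick projects the owner's location to screen space and moves the icon there, clamped inside viewport margins.
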(event Custom|OnComponentBeginOverlap_Event_0
  (params (OverlappedComponent :type Primitive%20Component%20Object%20Reference) (OtherActor :type Actor%20Object%20Reference) (OtherComp :type Primitive%20Component%20Object%20Reference) (OtherBodyIndex :type Integer) (bFromSweep :type Boolean) (SweepResult :type Hit%20Result%20Structure%20%28by%20ref%29))
  (bind _iconref (Variables|Default|GetIconRef))
  (Utilities|Casting|CastToSCPReduxCharacter_BP OtherActor)
  (Input|EnableInput (Components|GetOwner) (Game|GetPlayerController 0))
  (Variables|/Game/SCP/HUD/InteractIcon.InteractIcon_C|SetImage _iconref "/Game/SCP/HUD/Textures/handsymbol.handsymbol")
  (Widget|SetVisibility _iconref "HitTestInvisible")
  (Variables|Default|SetMoveInteractIcon true))

(event Custom|OnComponentEndOverlap_Event_0
  (params (OverlappedComponent :type Primitive%20Component%20Object%20Reference) (OtherActor :type Actor%20Object%20Reference) (OtherComp :type Primitive%20Component%20Object%20Reference) (OtherBodyIndex :type Integer))
  (Utilities|Casting|CastToSCPReduxCharacter_BP OtherActor)
  (Input|DisableInput (Components|GetOwner) (Game|GetPlayerController 0))
  (Widget|SetVisibility (Variables|Default|GetIconRef) "Hidden")
  (Variables|Default|SetMoveInteractIcon false))

(event EventBeginPlay
  (bind _returnvalue (Components|GetOwner))
  (bind _returnvalue_2 (Actor|GetComponentbyClass _returnvalue "/Script/Engine.CapsuleComponent"))
  (Collision|AssignOnComponentBeginOverlap _returnvalue_2 (delegate Custom|OnComponentBeginOverlap_Event_0))
  (Collision|AssignOnComponentEndOverlap _returnvalue_2 (delegate Custom|OnComponentEndOverlap_Event_0))
  (bind _asscpredux_character_bp (Utilities|Casting|CastToSCPReduxCharacter_BP (Game|Player|GetPlayerPawn 0)))
  (Variables|Default|SetIconRef (Variables|/Game/SCP/Character/SCPReduxCharacter_BP.SCPReduxCharacter_BP_C|GetInteractIcon _asscpredux_character_bp)))

(event EventTick
  (params (DeltaSeconds :type Float%20%28single-precision%29))
  (bind _returnvalue (Game|GetPlayerController 0))
  (bind _returnvalue_2 (Components|GetOwner))
  (bind _returnvalue_3 (Viewport|GetViewportSize))
  (bind _returnvalue_4 (Transformation|GetActorLocation _returnvalue_2))
  (bind _screenposition (Class|GameplayStatics|ProjectWorldtoScreen _returnvalue _returnvalue_4 false))
  (if (Variables|Default|GetMoveInteractIcon)
    (Class|Widget|SetRenderTranslation (Variables|Default|GetIconRef) (Math|Vector2D|MakeVector2D (- (Math|Float|Clamp(Float) (.x _screenposition) (* (.x _returnvalue_3) 0.1) (* (.x _returnvalue_3) 0.9)) 32.0) (- (Math|Float|Clamp(Float) (.y _screenposition) (* (.y _returnvalue_3) 0.15) (* (.y _returnvalue_3) 0.85)) 32.0)))))