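; Button Blueprint in the SCP game that handles buttons linked to a broken elevator, building on a parent button class.
; On BeginPlay, if its ParentDoor is valid and flagged as a broken elevator, it swaps the fail message for a broken-elevator notice.
; On Activate, it runs the parent logic first, then disables that door if the same flag is set.
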(event EventBeginPlay
  (bind _parentdoor (Variables|Default|GetParentDoor))
  (|CallParentFunction)
  (Utilities|IsValid _parentdoor
    (:Is%20Valid
      (if (Variables|/Game/SCP/Blueprints/Doors/DoorBase_BP.DoorBase_BP_C|GetIsBrokenElevator _parentdoor)
        (Variables|Default|SetFailMessage "The elevator appears to be broken.")))))

(event Collision|EventActorBeginOverlap
  (params (OtherActor :type Actor%20Object%20Reference)))

(event EventActivate
  (bind _parentdoor (Variables|Default|GetParentDoor))
  (|CallParentFunction)
  (Utilities|IsValid _parentdoor
    (:Is%20Valid
      (if (Variables|/Game/SCP/Blueprints/Doors/DoorBase_BP.DoorBase_BP_C|GetIsBrokenElevator _parentdoor)
        (Variables|/Game/SCP/Blueprints/Doors/DoorBase_BP.DoorBase_BP_C|SetDoorEnabled _parentdoor false)))))

(event EventTick
  (params (DeltaSeconds :type Float%20%28single-precision%29)))

(fn ConstructionScript
  (|CallParentFunction))