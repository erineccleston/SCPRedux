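; Base Blueprint for a two-panel sliding door that can start open and toggles between open and closed on each Open event.
; A FlipFlop plays or reverses a timeline that lerps both panels between start and end component positions.
; A DoOnce limits the open or close sound to once per movement, skipping the initial start-open motion.
; SetAsParent links child-actor door and two buttons, passing the clearance level to the door.
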(event Custom|Open
  (bind _returnvalue (Transformation|GetActorLocation))
  (bind _isa (Utilities|FlowControl|FlipFlop)
    (:A
      (bind _alpha (Timeline|Curve Play)
        (:Update
          (Transformation|SetRelativeLocation (Variables|Default|GetDoor2) (Math|Vector|Lerp(Vector) (Variables|Default|GetDoor2Start) (Variables|/Script/Engine.SceneComponent|GetRelativeLocation (Variables|Default|GetDoor2End)) _alpha) false false)
          (Transformation|SetRelativeLocation (Variables|Default|GetDoor1) (Math|Vector|Lerp(Vector) (Variables|Default|GetDoor1Start) (Variables|/Script/Engine.SceneComponent|GetRelativeLocation (Variables|Default|GetDoor1End)) _alpha) false false)
          (Utilities|FlowControl|DoOnce (Variables|Default|GetStartOpen) :!label _label
            (:Completed
              (if _isa
                (Audio|PlaySoundatLocation (Variables|Default|GetOpenSound) _returnvalue)
                (else
                  (Audio|PlaySoundatLocation (Variables|Default|GetCloseSound) _returnvalue))))))
        (:Finished
          (goto _label Reset))))
    (:B
      (Timeline|Curve Reverse))))

(event EventBeginPlay
  (bind _returnvalue (Transformation|GetActorLocation))
  (Variables|Default|SetDoor2Start (Variables|/Script/Engine.SceneComponent|GetRelativeLocation (Variables|Default|GetDoor2)))
  (Variables|Default|SetDoor1Start (Variables|/Script/Engine.SceneComponent|GetRelativeLocation (Variables|Default|GetDoor1)))
  (Components|Timeline|SetPlayRate (Variables|Default|GetCurve) (Variables|Default|GetPlayRate))
  (if (Variables|Default|GetStartOpen)
    (bind _isa (Utilities|FlowControl|FlipFlop)
      (:A
        (bind _alpha (Timeline|Curve Play)
          (:Update
            (Transformation|SetRelativeLocation (Variables|Default|GetDoor2) (Math|Vector|Lerp(Vector) (Variables|Default|GetDoor2Start) (Variables|/Script/Engine.SceneComponent|GetRelativeLocation (Variables|Default|GetDoor2End)) _alpha) false false)
            (Transformation|SetRelativeLocation (Variables|Default|GetDoor1) (Math|Vector|Lerp(Vector) (Variables|Default|GetDoor1Start) (Variables|/Script/Engine.SceneComponent|GetRelativeLocation (Variables|Default|GetDoor1End)) _alpha) false false)
            (Utilities|FlowControl|DoOnce (Variables|Default|GetStartOpen) :!label _label
              (:Completed
                (if _isa
                  (Audio|PlaySoundatLocation (Variables|Default|GetOpenSound) _returnvalue)
                  (else
                    (Audio|PlaySoundatLocation (Variables|Default|GetCloseSound) _returnvalue))))))
          (:Finished
            (goto _label Reset))))
      (:B
        (Timeline|Curve Reverse)))))

(fn ConstructionScript)

(fn SetasParent
  (params (Door :type Child%20Actor%20Component%20Object%20Reference) (Button1 :type Child%20Actor%20Component%20Object%20Reference) (Button2 :type Child%20Actor%20Component%20Object%20Reference) (ClearanceLevel :type Integer))
  (bind _asdoor_base_bp (Utilities|Casting|CastToDoorBase_BP (Variables|/Script/Engine.ChildActorComponent|GetChildActor Door)))
  (bind _output_get (LocalVariables|SetDoorRef _asdoor_base_bp))
  (Variables|DoorBase_BP_C|SetClearanceLevel _output_get ClearanceLevel)
  (bind _asbutton_base_bp (Utilities|Casting|CastToButtonBase_BP (Variables|/Script/Engine.ChildActorComponent|GetChildActor Button1)))
  (Variables|/Game/SCP/Blueprints/Buttons/ButtonBase_BP.ButtonBase_BP_C|SetParentDoor _asbutton_base_bp (LocalVariables|GetDoorRef))
  (bind _asbutton_base_bp_2 (Utilities|Casting|CastToButtonBase_BP (Variables|/Script/Engine.ChildActorComponent|GetChildActor Button2)))
  (Variables|/Game/SCP/Blueprints/Buttons/ButtonBase_BP.ButtonBase_BP_C|SetParentDoor _asbutton_base_bp_2 (LocalVariables|GetDoorRef)))