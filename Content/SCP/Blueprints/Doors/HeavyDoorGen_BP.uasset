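; HeavyDoorGen_BP is a heavy door Blueprint in the SCP game that pairs the door with two child-actor buttons.
; Its construction script runs the parent's, then casts Button1 and Button2 to ButtonBase_BP and sets itself as each one's ParentDoor.
; The second button is only linked if the first cast succeeds.
; The event graph holds only disabled placeholder events, so this file defines no door movement.
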(event EventBeginPlay
  (|CallParentFunction))

(event Collision|EventActorBeginOverlap
  (params (OtherActor :type Actor%20Object%20Reference)))

(event EventTick
  (params (DeltaSeconds :type Float%20%28single-precision%29)))

(fn ConstructionScript
  (|CallParentFunction)
  (bind _asbutton_base_bp (Utilities|Casting|CastToButtonBase_BP (Variables|/Script/Engine.ChildActorComponent|GetChildActor (Variables|Default|GetButton1))))
  (Variables|/Game/SCP/Blueprints/Buttons/ButtonBase_BP.ButtonBase_BP_C|SetParentDoor _asbutton_base_bp self)
  (bind _asbutton_base_bp_2 (Utilities|Casting|CastToButtonBase_BP (Variables|/Script/Engine.ChildActorComponent|GetChildActor (Variables|Default|GetButton2))))
  (Variables|/Game/SCP/Blueprints/Buttons/ButtonBase_BP.ButtonBase_BP_C|SetParentDoor _asbutton_base_bp_2 self))