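; SCP-1162 interactable that trades a random item from the player's inventory for a new one when activated.
; The result of RemoveRandom selects either a harmless exchange sound or a horror sound with player damage and increased bleed rate.
; Both outcomes spawn an ItemBase_BP at ItemSpawn with random yaw, then set its type randomly from OutputItems.
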(event EventBeginPlay)

(event Collision|EventActorBeginOverlap
  (params (OtherActor :type Actor%20Object%20Reference)))

(event EventTick
  (params (DeltaSeconds :type Float%20%28single-precision%29))
  (|CallParentFunction DeltaSeconds))

(event EventActivate
  (bind _playerchar (CallFunction|GetPlayerChar))
  (bind _returnvalue (Transformation|GetActorLocation))
  (bind _outputitems (Variables|Default|GetOutputItems))
  (bind _invempty (Default|RemoveRandom (CallFunction|GetPlayerInv)))
  (if _invempty
    (Audio|PlaySoundatLocation "/Game/SCP/Maps/Sounds/1162/1162Horror.1162Horror" _returnvalue)
    (Game|Damage|ApplyDamage _playerchar 5e+01 0 0 "/Game/SCP/Blueprints/DamageTypes/1162Damage.1162Damage_C")
    (Variables|/Game/SCP/Character/SCPReduxCharacter_BP.SCPReduxCharacter_BP_C|SetBleedRate _playerchar (+ (Variables|/Game/SCP/Character/SCPReduxCharacter_BP.SCPReduxCharacter_BP_C|GetBleedRate _playerchar) 2.5))
    (else
      (Audio|PlaySoundatLocation "/Game/SCP/Maps/Sounds/1162/1162Exchange.1162Exchange" _returnvalue)))
  (bind _returnvalue_2 (Game|SpawnActorfromClass "/Game/SCP/Blueprints/BaseClasses/ItemBase_BP.ItemBase_BP_C" (Math|Transform|MakeTransform (Transformation|GetWorldLocation (Variables|Default|GetItemSpawn)) (Math|Rotator|MakeRotator 0.0 0.0 (Math|Random|RandomFloatinRange 0.0 3.6e+02)) "1,1,1") "AdjustIfPossibleButAlwaysSpawn" 0 "NewEnumerator59" 0))
  (Default|SetType _returnvalue_2 (Utilities|Array|Get(acopy) _outputitems (Math|Random|RandomIntegerinRange 0 (- (Utilities|Array|Length _outputitems) 1)))))

(fn ConstructionScript)