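; Grabbable knob interactable, apparently for SCP-914, that turns with the player's rotation and snaps to detents.
; While grabbed, it applies the player's rotation delta as local rotation to Body, mapping yaw to pitch, only while Body's up vector Z stays above a small threshold.
; SettlingBehavior plays a Settle timeline that lerps world pitch to the nearest fixed step along the shortest path, keeping roll and yaw.
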(event EventBeginPlay)

(event Collision|EventActorBeginOverlap
  (params (OtherActor :type Actor%20Object%20Reference)))

(event EventTick
  (params (DeltaSeconds :type Float%20%28single-precision%29))
  (|CallParentFunction DeltaSeconds))

(event EventWhileGrabbed
  (bind _playerrotdelta (Variables|Default|GetPlayerRotDelta))
  (if (> (.z (Math|Vector|GetUpVector (Variables|Default|GetBody))) 0.075)
    (Transformation|AddLocalRotation (Variables|Default|GetBody) (Math|Rotator|MakeRotator (.roll _playerrotdelta) (.yaw _playerrotdelta) (.pitch _playerrotdelta)) false false)))

(event EventSettlingBehavior
  (Variables|Default|SetLocalWorldRot (Transformation|GetWorldRotation (Variables|Default|GetBody)))
  (bind _alpha (Timeline|Settle PlayFromStart)
    (:Update
      (Transformation|SetWorldRotation (Variables|Default|GetBody) (Math|Rotator|Lerp(Rotator) (Variables|Default|GetLocalWorldRot) (Math|Rotator|MakeRotator (.roll (Variables|Default|GetLocalWorldRot)) (* (Math|Float|Round (/ (.pitch (Variables|Default|GetLocalWorldRot)) 42.5)) 42.5) (.yaw (Variables|Default|GetLocalWorldRot))) _alpha true) false false))))

(fn ConstructionScript
  (|CallParentFunction))