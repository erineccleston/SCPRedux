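; Base Blueprint for interactable objects in the SCP game, providing Activate and Deactivate events.
; Activate plays the interact sound at the actor's location, while Deactivate is empty.
; GetHandsOld, named as an older version, returns Up/Down/Left/Right hand flags by casting self to child classes.
; Levers set up and down, while the 914 key and knob set left and right.
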(event Custom|Activate
  (Audio|PlaySoundatLocation (Variables|Default|GetInteractSound) (Transformation|GetActorLocation)))

(event Custom|Deactivate)

(event EventBeginPlay)

(event Collision|EventActorBeginOverlap
  (params (OtherActor :type Actor%20Object%20Reference)))

(event EventTick
  (params (DeltaSeconds :type Float%20%28single-precision%29)))

(fn ConstructionScript)

(fn GetHandsOld
  (bind _self self)
  (Utilities|FlowControl|Sequence
    (:then_0
      (Utilities|Casting|CastToLever_BP _self
        (:then
          (LocalVariables|SetU true)
          (LocalVariables|SetD true))
        (:CastFailed
          (Utilities|Casting|CastTo914Key_BP _self
            (:then
              (LocalVariables|SetL true)
              (LocalVariables|SetR true))
            (:CastFailed
              (Utilities|Casting|CastTo914Knob_BP _self)
              (LocalVariables|SetL true)
              (LocalVariables|SetR true))))))
    (:then_1
      (return (LocalVariables|GetU) (LocalVariables|GetD) (LocalVariables|GetL) (LocalVariables|GetR)))))