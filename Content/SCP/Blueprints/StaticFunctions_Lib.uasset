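; StaticFunctions_Lib is a set of shared helper functions for doors and randomness in the SCP game.
; InitDoor sets a child-actor door's clearance level and cross-links it with up to two button child actors.
; AInBChance rolls an A-in-B chance from a stream seeded by the current millisecond.
; PseudoHash folds a string's character codes into an integer, and GlobalRand returns the GameInstance_BP's GlobalSeed unchanged.
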(fn InitDoor
  (params (Door :type Child%20Actor%20Component%20Object%20Reference) (Button1 :type Child%20Actor%20Component%20Object%20Reference) (Button2 :type Child%20Actor%20Component%20Object%20Reference) (Level :type Integer))
  (Utilities|FlowControl|Sequence
    (:then_0
      (bind _asdoor_base_bp (Utilities|Casting|CastToDoorBase_BP (Variables|/Script/Engine.ChildActorComponent|GetChildActor Door)))
      (bind _output_get (LocalVariables|SetDoorRef _asdoor_base_bp))
      (Variables|/Game/SCP/Blueprints/BaseClasses/DoorBase_BP.DoorBase_BP_C|SetClearanceLevel _output_get Level))
    (:then_1
      (Utilities|IsValid Button1
        (:Is%20Valid
          (bind _asbutton_base_bp (Utilities|Casting|CastToButtonBase_BP (Variables|/Script/Engine.ChildActorComponent|GetChildActor Button1)))
          (Utilities|Array|AddUnique (Variables|/Game/SCP/Blueprints/BaseClasses/ButtonBase_BP.ButtonBase_BP_C|GetParents _asbutton_base_bp) (LocalVariables|GetDoorRef))
          (Utilities|Array|AddUnique (Variables|/Game/SCP/Blueprints/BaseClasses/DoorBase_BP.DoorBase_BP_C|GetChildButtons (LocalVariables|GetDoorRef)) _asbutton_base_bp))))
    (:then_2
      (Utilities|IsValid Button2
        (:Is%20Valid
          (bind _asbutton_base_bp_2 (Utilities|Casting|CastToButtonBase_BP (Variables|/Script/Engine.ChildActorComponent|GetChildActor Button2)))
          (Utilities|Array|AddUnique (Variables|/Game/SCP/Blueprints/BaseClasses/ButtonBase_BP.ButtonBase_BP_C|GetParents _asbutton_base_bp_2) (LocalVariables|GetDoorRef))
          (Utilities|Array|AddUnique (Variables|/Game/SCP/Blueprints/BaseClasses/DoorBase_BP.DoorBase_BP_C|GetChildButtons (LocalVariables|GetDoorRef)) _asbutton_base_bp_2))))))

(fn AinBChance
  (params (A :type Integer) (B :type Integer))
  (return (<= (Math|Random|RandomIntegerinRangefromStream 1 B (Math|Random|MakeRandomStream (Math|DateTime|GetMillisecond (Math|DateTime|Now)))) A)))

(fn PseudoHash
  (params (String :type String))
  (for _index (range 0 (Utilities|String|Len String))
    (bind _output_get (LocalVariables|SetLocalInt (+ (LocalVariables|GetLocalInt) (Utilities|String|GetCharacterasNumber String _index))))
    (LocalVariables|SetLocalInt (* _output_get 10)))
  (return (LocalVariables|GetLocalInt)))

(fn GlobalRand
  (return (Variables|/Game/SCP/Character/GameInstance_BP.GameInstance_BP_C|GetGlobalSeed (.AsGame%20Instance%20BP (Utilities|Casting|CastToGameInstance_BP (Game|GetGameInstance))))))