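; Security camera Blueprint that sweeps its view from side to side and renders it to a texture.
; On BeginPlay, a timeline lerps the camera base's relative yaw between positive and negative max yaw, reusing its world roll and pitch.
; The construction script creates a render target per camera, feeds it to the scene capture component and caps capture view distance for performance.
; Despite the Tracking name, it contains no target-following logic.
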(event EventBeginPlay
  (bind _camera_max_yaw (Variables|Scanning|GetCamera%20Max%20Yaw))
  (bind _camera_base (Variables|BP_Security_Camera_Tracking|GetCamera%20base))
  (bind _returnvalue (Transformation|GetWorldRotation _camera_base))
  (bind _scan_rotation (Timeline|Scan%20Rot%20Timeline Play) ; Camera animation of yaw rotation
    (:Update
      (Transformation|SetRelativeRotation (Variables|BP_Security_Camera_Tracking|GetCamera%20base) (Math|Rotator|Lerp(Rotator) (Math|Rotator|MakeRotator (.roll _returnvalue) (.pitch _returnvalue) _camera_max_yaw) (Math|Rotator|MakeRotator (.roll _returnvalue) (.pitch _returnvalue) (* _camera_max_yaw -1.0)) _scan_rotation) false false))))

(fn ConstructionScript
  (bind _scenecapture (Variables|BP_Security_Camera_Tracking|GetSceneCapture))
  (bind _returnvalue (Rendering|CreateRenderTarget2D 512 512))
  (bind _output_get (Variables|RenderTarget|SetScene%20Capture%20Texture _returnvalue))
  (Variables|/Script/Engine.SceneCaptureComponent2D|SetTextureTarget _scenecapture _output_get)
  (Variables|/Script/Engine.SceneCaptureComponent|SetMaxViewDistanceOverride _scenecapture (Variables|RenderTarget|GetScene%20Capture%20View%20Distance))
  (Rendering|SetVisibility (Variables|BP_Security_Camera_Tracking|GetSceneCapture) true false) ; Turn scene capture on or off
)