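; CandyBowl_BP is an interactable candy bowl that punishes the player for taking more than two candies.
; Activate puts one of three random candy types in an empty inventory slot, or reports a full inventory.
; Past the limit, it spawns two mirrored items at the player's feet, disables interaction, deals damage and increases bleeding.
; The first character to enter its capsule triggers a one-time warning message.
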(event EventBndEvtCapsuleK2NodeComponentBoundEvent0ComponentBeginOverlapSignatureDelegateSignature
  (params (OverlappedComponent :type Primitive%20Component%20Object%20Reference) (OtherActor :type Actor%20Object%20Reference) (OtherComp :type Primitive%20Component%20Object%20Reference) (OtherBodyIndex :type Integer) (bFromSweep :type Boolean) (SweepResult :type Hit%20Result%20Structure%20%28by%20ref%29))
  (|CallParentFunction OverlappedComponent OtherActor OtherComp OtherBodyIndex bFromSweep SweepResult)
  (bind _asscpredux_character_bp (Utilities|Casting|CastToSCPReduxCharacter_BP OtherActor))
  (Utilities|FlowControl|DoOnce false
    (:Completed
      (Default|QueueMessage _asscpredux_character_bp "take no more than two, please!!"))))

(event EventActivate
  (bind _playerchar (CallFunction|GetPlayerChar))
  (bind _playerchar_2 (CallFunction|GetPlayerChar))
  (bind _playerchar_3 (CallFunction|GetPlayerChar))
  (bind _playerchar_4 (CallFunction|GetPlayerChar))
  (bind _playerchar_5 (CallFunction|GetPlayerChar))
  (bind _returnvalue (Transformation|GetActorRightVector _playerchar_4))
  (bind _returnvalue_2 (Transformation|GetActorRightVector _playerchar))
  (bind _inventory (Variables|/Game/SCP/Character/SCPReduxCharacter_BP.SCPReduxCharacter_BP_C|GetInventory _playerchar_3))
  (bind _returnvalue_3 (Utilities|Array|FindItem _inventory "NewEnumerator59"))
  (bind _returnvalue_4 (* _returnvalue 5e+01))
  (bind _returnvalue_5 (* _returnvalue_2 -5e+01))
  (if (>= _returnvalue_3 0)
    (Audio|PlaySoundatLocation "/Game/SCP/Blueprints/Sounds/PickItem0.PickItem0" (Transformation|GetActorLocation))
    (bind _candy (CallFunction|RandomCandy))
    (Utilities|Array|SetArrayElem (Variables|/Game/SCP/Character/SCPReduxCharacter_BP.SCPReduxCharacter_BP_C|GetInventory (CallFunction|GetPlayerChar)) _returnvalue_3 _candy)
    (bind _result (Math|Integer|IncrementInt (Variables|Default|GetCandiesTaken))
      (:%20%20
        (if (> _result 2)
          (bind _returnvalue_6 (Game|SpawnActorfromClass "/Game/SCP/Blueprints/ItemBase_BP.ItemBase_BP_C" (Math|Transform|MakeTransform (+ (Transformation|GetActorLocation _playerchar_4) (Math|Vector|MakeVector (.x _returnvalue_4) (.y _returnvalue_4) (* (Components|Capsule|GetScaledCapsuleHalfHeight (Variables|/Script/Engine.Character|GetCapsuleComponent _playerchar_4)) -1.0))) (Math|Rotator|CombineRotators (Transformation|GetActorRotation _playerchar_4) "0,180.000000, 0") "-1.000000,1.000000,1") "AdjustIfPossibleButAlwaysSpawn" 0 "NewEnumerator59" 0))
          (Default|SetType _returnvalue_6 "NewEnumerator30")
          (bind _returnvalue_7 (Game|SpawnActorfromClass "/Game/SCP/Blueprints/ItemBase_BP.ItemBase_BP_C" (Math|Transform|MakeTransform (+ (Transformation|GetActorLocation _playerchar) (Math|Vector|MakeVector (.x _returnvalue_5) (.y _returnvalue_5) (* (Components|Capsule|GetScaledCapsuleHalfHeight (Variables|/Script/Engine.Character|GetCapsuleComponent _playerchar)) -1.0))) (Transformation|GetActorRotation _playerchar) "1.000000,1.000000,1.000000") "AdjustIfPossibleButAlwaysSpawn" 0 "NewEnumerator59" 0))
          (Default|SetType _returnvalue_7 "NewEnumerator30")
          (Variables|/Game/SCP/Character/SCPReduxCharacter_BP.SCPReduxCharacter_BP_C|SetCanInteract _playerchar_5 false)
          (Widget|RemovefromParent (Variables|/Game/SCP/Character/SCPReduxCharacter_BP.SCPReduxCharacter_BP_C|GetInteractIcon _playerchar_5))
          (Audio|PlaySound2D "/Game/SCP/Character/Sounds/Damage4.Damage4")
          (Game|Damage|ApplyDamage _playerchar_2 5e+01 0 0 "/Game/SCP/Blueprints/DamageTypes/CandyBowlDamage.CandyBowlDamage_C")
          (Variables|/Game/SCP/Character/SCPReduxCharacter_BP.SCPReduxCharacter_BP_C|SetBleedRate _playerchar_2 (+ (Variables|/Game/SCP/Character/SCPReduxCharacter_BP.SCPReduxCharacter_BP_C|GetBleedRate _playerchar_2) 2.5)))))
    (else
      (Default|QueueMessage (CallFunction|GetPlayerChar) "You cannot carry any more items."))))

(fn ConstructionScript)

(fn RandomCandy
  (switch int (Math|Random|RandomIntegerinRange 0 2)
    (:0
      (return "NewEnumerator71"))
    (:1
      (return "NewEnumerator72"))
    (:2
      (return "NewEnumerator73"))))